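; Art placement Blueprint that scatters static meshes along its Path spline in the construction script.
; Each InstanceData entry spawns evenly spaced, separate Static Mesh Components despite the "Instance" name, aligned to the spline's right and up vectors.
; Composed transforms layer offsets, index-seeded random jitter in position, rotation and scale, plus a scale taper around a bias point.
; EnableCollisions sets collision only on the Path component, not the spawned meshes.
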(event EventBeginPlay)

(event Collision|EventActorBeginOverlap
  (params (OtherActor :type Actor%20Object%20Reference)))

(event EventTick
  (params (DeltaSeconds :type Float%20%28single-precision%29)))

(fn ConstructionScript
  (bind _path (Variables|Default|GetPath))
  (bind _path_2 (Variables|Default|GetPath))
  (Utilities|FlowControl|Sequence
    (:then_0
      ;[1 1 1] Path Variables
      (LocalVariables|SetLocal_SplineLength (Spline|GetSplineLength _path))
      (LocalVariables|SetLocal_SplineTransform (Transformation|GetWorldTransform _path)))
    (:then_1
      (for _array_element (Variables|Default|GetInstanceData)
        ;[1 1 1] Local Variables
        (LocalVariables|SetLocal_Mesh (.staticmesh (Utilities|Array|Get(acopy) (Utilities|Array|MakeArray _array_element))))
        (LocalVariables|SetLocal_Count (.count (Utilities|Array|Get(acopy) (Utilities|Array|MakeArray _array_element))))
        (LocalVariables|SetLocal_Spread (/ (LocalVariables|GetLocal_SplineLength) (Math|Conversions|ToFloat(Integer) (- (.count (Utilities|Array|Get(acopy) (Utilities|Array|MakeArray _array_element))) 1))))
        (LocalVariables|SetLocal_RandomLocation (.randomlocation (Utilities|Array|Get(acopy) (Utilities|Array|MakeArray _array_element))))
        (LocalVariables|SetLocal_PositionOffset (.position (Utilities|Array|Get(acopy) (Utilities|Array|MakeArray _array_element))))
        (LocalVariables|SetLocal_RandPosition (.randposition (Utilities|Array|Get(acopy) (Utilities|Array|MakeArray _array_element))))
        (LocalVariables|SetLocal_CurrentRotation (.rotation (Utilities|Array|Get(acopy) (Utilities|Array|MakeArray _array_element))))
        (LocalVariables|SetLocal_RandRotation (.randrotation (Utilities|Array|Get(acopy) (Utilities|Array|MakeArray _array_element))))
        (LocalVariables|SetLocal_CurrentScale (.scale (Utilities|Array|Get(acopy) (Utilities|Array|MakeArray _array_element))))
        (LocalVariables|SetLocal_RandScale (.randscale (Utilities|Array|Get(acopy) (Utilities|Array|MakeArray _array_element))))
        (LocalVariables|SetLocal_LocationOffset (.locationoffset (Utilities|Array|Get(acopy) (Utilities|Array|MakeArray _array_element))))
        (LocalVariables|SetLocal_RemoveLast (.removelast (Utilities|Array|Get(acopy) (Utilities|Array|MakeArray _array_element))))
        (LocalVariables|SetLocal_LastIndex (- (LocalVariables|GetLocal_Count) (select (LocalVariables|GetLocal_RemoveLast) 2 1)))
        (LocalVariables|SetLocal_Seed (.seed (Utilities|Array|Get(acopy) (Utilities|Array|MakeArray _array_element))))
        (LocalVariables|SetLocal_Taper (.taper (Utilities|Array|Get(acopy) (Utilities|Array|MakeArray _array_element))))
        (LocalVariables|SetLocal_TaperBias (.taperbias (Utilities|Array|Get(acopy) (Utilities|Array|MakeArray _array_element))))
        (for _index (range 0 (LocalVariables|GetLocal_LastIndex))
          (bind _output_get (LocalVariables|SetLocal_CurIndex _index))
          (LocalVariables|SetLocal_RandStream (Math|Random|MakeRandomStream (+ (* (LocalVariables|GetLocal_CurIndex) 3) (LocalVariables|GetLocal_Seed))))
          (LocalVariables|SetLocal_DistanceAlongSpline (+ (* _output_get (LocalVariables|GetLocal_Spread)) (Math|Random|RandomFloatinRangefromStream (* (LocalVariables|GetLocal_RandomLocation) -1.0) (LocalVariables|GetLocal_RandomLocation) (LocalVariables|GetLocal_RandStream)) (LocalVariables|GetLocal_LocationOffset)))
          (Utilities|FlowControl|Sequence
            (:then_0
              (bind _returnvalue (AddComponent|AddStaticMeshComponent false))
              (Components|StaticMesh|SetStaticMesh _returnvalue (LocalVariables|GetLocal_Mesh))
              (LocalVariables|SetLocal_StaticMeshComponent _returnvalue))
            (:then_1
              (LocalVariables|SetLocal_FinalPosition (Spline|GetLocationatDistanceAlongSpline (Variables|Default|GetPath) (LocalVariables|GetLocal_DistanceAlongSpline) "Local")))
            (:then_2
              (LocalVariables|SetLocal_FinalRotation (Class|KismetMathLibrary|MakeRotfromYZ (Class|SplineComponent|GetRightVectoratDistanceAlongSpline _path_2 (LocalVariables|GetLocal_DistanceAlongSpline) "Local") (Class|SplineComponent|GetUpVectoratDistanceAlongSpline _path_2 (LocalVariables|GetLocal_DistanceAlongSpline) "Local"))))
            (:then_3
              ;[1 1 1] World Transform
              (Transformation|SetWorldTransform (LocalVariables|GetLocal_StaticMeshComponent) (Math|Transform|ComposeTransforms (Math|Transform|ComposeTransforms (Math|Transform|ComposeTransforms (Math|Transform|MakeTransform "0, 0, 0" (Math|Rotator|MakeRotator (.X (Math|Vector|BreakVector (LocalVariables|GetLocal_CurrentRotation))) (.Y (Math|Vector|BreakVector (LocalVariables|GetLocal_CurrentRotation))) (.Z (Math|Vector|BreakVector (LocalVariables|GetLocal_CurrentRotation))))) (Math|Transform|MakeTransform "0, 0, 0" (Math|Rotator|MakeRotator (Math|Random|RandomFloatinRangefromStream (* (.X (Math|Vector|BreakVector (LocalVariables|GetLocal_RandRotation))) -1.0) (.X (Math|Vector|BreakVector (LocalVariables|GetLocal_RandRotation))) (LocalVariables|GetLocal_RandStream)) (Math|Random|RandomFloatinRangefromStream (* (.Y (Math|Vector|BreakVector (LocalVariables|GetLocal_RandRotation))) -1.0) (.Y (Math|Vector|BreakVector (LocalVariables|GetLocal_RandRotation))) (LocalVariables|GetLocal_RandStream)) (Math|Random|RandomFloatinRangefromStream (* (.Z (Math|Vector|BreakVector (LocalVariables|GetLocal_RandRotation))) -1.0) (.Z (Math|Vector|BreakVector (LocalVariables|GetLocal_RandRotation))) (LocalVariables|GetLocal_RandStream))))) (Math|Transform|ComposeTransforms (Math|Transform|ComposeTransforms (Math|Transform|MakeTransform (LocalVariables|GetLocal_PositionOffset) "0, 0, 0" (+ (+ (Math|Vector|MakeVector (Math|Random|RandomFloatinRangefromStream (* (.X (Math|Vector|BreakVector (LocalVariables|GetLocal_RandScale))) -1.0) (.X (Math|Vector|BreakVector (LocalVariables|GetLocal_RandScale))) (LocalVariables|GetLocal_RandStream)) (Math|Random|RandomFloatinRangefromStream (* (.Y (Math|Vector|BreakVector (LocalVariables|GetLocal_RandScale))) -1.0) (.Y (Math|Vector|BreakVector (LocalVariables|GetLocal_RandScale))) (LocalVariables|GetLocal_RandStream)) (Math|Random|RandomFloatinRangefromStream (* (.Z (Math|Vector|BreakVector (LocalVariables|GetLocal_RandScale))) -1.0) (.Z (Math|Vector|BreakVector (LocalVariables|GetLocal_RandScale))) (LocalVariables|GetLocal_RandStream))) "1.000000,1.000000,1.000000") (* (LocalVariables|GetLocal_Taper) (Math|Float|Absolute(Float) (- (/ (Math|Conversions|ToFloat(Integer) (LocalVariables|GetLocal_CurIndex)) (Math|Conversions|ToFloat(Integer) (LocalVariables|GetLocal_Count))) (LocalVariables|GetLocal_TaperBias)))))) (Math|Transform|MakeTransform (Math|Vector|MakeVector (Math|Random|RandomFloatinRangefromStream (* (.X (Math|Vector|BreakVector (LocalVariables|GetLocal_RandPosition))) -1.0) (.X (Math|Vector|BreakVector (LocalVariables|GetLocal_RandPosition))) (LocalVariables|GetLocal_RandStream)) (Math|Random|RandomFloatinRangefromStream (* (.Y (Math|Vector|BreakVector (LocalVariables|GetLocal_RandPosition))) -1.0) (.Y (Math|Vector|BreakVector (LocalVariables|GetLocal_RandPosition))) (LocalVariables|GetLocal_RandStream)) (Math|Random|RandomFloatinRangefromStream (* (.Z (Math|Vector|BreakVector (LocalVariables|GetLocal_RandPosition))) -1.0) (.Z (Math|Vector|BreakVector (LocalVariables|GetLocal_RandPosition))) (LocalVariables|GetLocal_RandStream))))) (Math|Transform|MakeTransform (LocalVariables|GetLocal_FinalPosition) (LocalVariables|GetLocal_FinalRotation) (LocalVariables|GetLocal_CurrentScale)))) (LocalVariables|GetLocal_SplineTransform)) false false))))))
    (:then_2
      ;[1 1 1] Collisions
      (Collision|SetCollisionEnabled (Variables|Default|GetPath) (select (Variables|Default|GetEnable%20Collisions) "QueryAndPhysics" "NoCollision")))))