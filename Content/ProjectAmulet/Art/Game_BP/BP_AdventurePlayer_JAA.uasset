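; BP_AdventurePlayer_JAA is a player character Blueprint handling movement, look, sprint, jump and crouch input.
; Axis events drive movement along the actor's forward and right vectors, plus controller yaw and pitch, while sprint swaps walk speed and crouch toggles through a FlipFlop.
; Movement starts a head-bob camera shake scaled by the axis value, and jumping plays a world camera shake, with a separate Jump event setting jump velocity.
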(event Input|ActionEvents|InputActionJump
  (params (Key :type Key%20Structure))
  (:Pressed
    (Variables|/Script/Engine.CharacterMovementComponent|SetJumpZVelocity (Variables|Character|GetCharacterMovement) (Variables|Default|GetJumpHeight))))

(event Input|ActionEvents|InputActionCrouch
  (params (Key :type Key%20Structure))
  (:Pressed
    (Utilities|FlowControl|FlipFlop
      (:A
        (Character|Crouch))
      (:B
        (Character|UnCrouch)))))

(event Input|ActionEvents|InputActionSprint
  (params (Key :type Key%20Structure))
  (bind _charactermovement (Variables|Character|GetCharacterMovement))
  (:Pressed
    (Variables|/Script/Engine.CharacterMovementComponent|SetMaxWalkSpeed _charactermovement (Variables|Default|GetRun%20Speed)))
  (:Released
    (Variables|/Script/Engine.CharacterMovementComponent|SetMaxWalkSpeed _charactermovement (Variables|Default|GetWalk%20Speed))))

(event Input|ActionEvents|InputActionJump
  (params (Key :type Key%20Structure))
  (:Pressed
    (Character|Jump)
    (Camera|PlayWorldCameraShake "/Game/ProjectAmulet/Art/Game_BP/BP_Jump_JAA.BP_Jump_JAA_C" (Transformation|GetActorLocation) 0.0 5e+02)))

(event Input|AxisEvents|InputAxisFrontBack
  (params (AxisValue :type Float%20%28single-precision%29))
  (Pawn|Input|AddMovementInput (Math|Vector|GetForwardVector (Transformation|GetActorRotation)) AxisValue false)
  (Game|Feedback|ClientStartCameraShake (Game|GetPlayerController 0) "/Game/ProjectAmulet/Art/Game_BP/BP_HeadBob_JAA.BP_HeadBob_JAA_C" AxisValue "CameraLocal" "0, 0, 0"))

(event Input|AxisEvents|InputAxisSidetoSide
  (params (AxisValue :type Float%20%28single-precision%29))
  (Pawn|Input|AddMovementInput (Math|Vector|GetRightVector (Transformation|GetActorRotation)) AxisValue false)
  (Game|Feedback|ClientStartCameraShake (Game|GetPlayerController 0) "/Game/ProjectAmulet/Art/Game_BP/BP_HeadBob_JAA.BP_HeadBob_JAA_C" AxisValue "CameraLocal" "0, 0, 0"))

(event Input|AxisEvents|InputAxisTurn
  (params (AxisValue :type Float%20%28single-precision%29))
  (Pawn|Input|AddControllerYawInput AxisValue))

(event Input|AxisEvents|InputAxisLookupDown
  (params (AxisValue :type Float%20%28single-precision%29))
  (Pawn|Input|AddControllerPitchInput AxisValue))

(fn ConstructionScript)

(fn NewFunction0)