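; Game State for a two-team attack/defend match, tracking rounds, scores, amulet points and the round timer.
; Timer expiry scores for defenders; each score checks for a two-win victory or swaps sides, resets amulets and starts the next pre-round with BP_MatchGameMode, the third being overtime.
; Event dispatchers feed timer, score, life and objective updates out, while local functions show round and team-specific victory screens and OnRep_AttackingTeam rechecks player freezing.
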(event Custom|Spawn%20Round%20Screen%20%28Multi%29
  (CallFunction|SpawnRoundScreen))

(event Custom|PreRound)

(event Custom|ScoreUpdate
  ;[1 1 1] Event Dispatcher events
  (Default|CallUpdateScore))

(event Custom|Timers
  (params (Sec :type Integer) (Min :type Integer))
  ;[1 1 1] Event Dispatcher events
  (Default|CallUpdateTimers Sec Min))

(event Custom|AlphaLifeCount
  ;[1 1 1] Event Dispatcher events
  (Default|CallUpdateAlphaLives))

(event Custom|BravoLifeCount
  ;[1 1 1] Event Dispatcher events
  (Default|CallUpdateBravoLives))

(event Custom|MatchEnd
  (params (Winner :type BP_ETeam%20Enum :default "NewEnumerator0"))
  ;[1 1 1] Event Dispatcher events
  (CallFunction|EndGame Winner))

(event Custom|ResetRound
  ;[1 1 1] Event Dispatcher events
  (Default|CallRoundReset))

(event Custom|AmuletPoints
  ;[1 1 1] Event Dispatcher events
  (Default|CallUpdateAmuletPoints))

(event Custom|Update%20Objective
  (bind _asbp_match_player_state (Utilities|Casting|CastToBP_MatchPlayerState (Variables|/Script/Engine.Pawn|GetPlayerState (Game|GetPlayerCharacter 0))))
  (Default|CallUpateObjective (Variables|/Game/ProjectAmulet/Maps/BP_MatchPlayerState.BP_MatchPlayerState_C|GetTeam _asbp_match_player_state) (Variables|Round|GetAttackingTeam) (== (Variables|Round|GetCurrentRound) 2)))

(event EventBeginPlay
  (Networking|SwitchHasAuthority
    (:Authority
      (CallFunction|SpawnRoundScreen(Multi)))))

(event EventTick
  (params (DeltaSeconds :type Float%20%28single-precision%29))
  (bind (_minutes _seconds) (CallFunction|GetRemainingTimeMinSec))
  (Networking|SwitchHasAuthority
    (:Authority
      (CallFunction|Timers _seconds _minutes))))

(fn ConstructionScript)

(fn EarnAttackerPoint
  (CallFunction|AddScore (Utilities|Enum|Equal(Enum) (Variables|Round|GetAttackingTeam) "NewEnumerator0")))

(fn EarnDefenderPoint
  (CallFunction|AddScore (Utilities|Enum|Equal(Enum) (Variables|Round|GetAttackingTeam) "NewEnumerator1")))

(fn SwapTeams
  (Development|PrintString "Teams Swaped")
  (switch Utilities|FlowControl|Switch|SwitchonBP_ETeam (Variables|Round|GetAttackingTeam)
    (:NewEnumerator0
      (Variables|Round|SetAttackingTeam "NewEnumerator1"))
    (:NewEnumerator1
      (Variables|Round|SetAttackingTeam "NewEnumerator0")))
  (bind _asbp_match_game_mode (Utilities|Casting|CastToBP_MatchGameMode (Game|GetGameMode)))
  (Default|SwapTeams _asbp_match_game_mode)
  (CallFunction|ResetAmuletSystem)
  (Default|ResetPlayerLocations _asbp_match_game_mode)
  (Variables|Round|SetCurrentAmuletPoints (Variables|Round|GetStartingAmuletPoints))
  (CallFunction|AmuletPoints))

(fn GetRemainingTimeMinSec
  (bind _timer (Variables|Round|GetTimer))
  (bind _returnvalue (Utilities|Time|GetTimerRemainingTimebyHandle _timer))
  (bind (_remainder _returnvalue_2) (Math|Float|Division(WholeandRemainder) _returnvalue 6e+01))
  (return _returnvalue_2 (Math|Float|Truncate _remainder)))

(fn IncrementRound
  (CallFunction|SwapTeams)
  (Math|Integer|IncrementInt (Variables|Round|GetCurrentRound)
    (:%20%20
      (bind _asbp_match_game_mode (Utilities|Casting|CastToBP_MatchGameMode (Game|GetGameMode)))
      (Default|StartPreRound _asbp_match_game_mode)
      (CallFunction|SpawnRoundScreen(Multi)))))

(fn UseAmuletPoints
  (params (PointsToUse :type Integer))
  (if (<= PointsToUse (Variables|Round|GetCurrentAmuletPoints))
    (Variables|Round|SetCurrentAmuletPoints (- (Variables|Round|GetCurrentAmuletPoints) PointsToUse))
    (CallFunction|AmuletPoints))
  (return (<= PointsToUse (Variables|Round|GetCurrentAmuletPoints))))

(fn AddScore
  (params (IsAlpha :type Boolean))
  (if IsAlpha
    (Math|Integer|IncrementInt (Variables|Score|GetAlphaWins)
      (:%20%20
        _))
    (else
      (Math|Integer|IncrementInt (Variables|Score|GetBravoWins)
        (:%20%20
          _))))
  (CallFunction|ScoreUpdate)
  (CallFunction|VictoryCheck))

(fn StartPreRoundTimer
  (params (Duration :type Float%20%28single-precision%29) (FunctionName :type String))
  (bind _asbp_match_game_mode (Utilities|Casting|CastToBP_MatchGameMode (Game|GetGameMode)))
  (bind _returnvalue (Utilities|Time|SetTimerbyFunctionName _asbp_match_game_mode FunctionName Duration))
  (Variables|Round|SetTimer _returnvalue)
  (CallFunction|UpdateObjective))

(fn StartRoundTimer
  (params (Duration :type Float%20%28single-precision%29))
  (bind _returnvalue (Utilities|Time|SetTimerbyFunctionName self "Earn Defender Point" Duration))
  (Variables|Round|SetTimer _returnvalue))

(fn EndGame
  (params (Winner :type BP_ETeam%20Enum :default "NewEnumerator0"))
  (bind _returnvalue (Game|GetPlayerController 0))
  (bind _returnvalue_2 (Game|GetPlayerController 0))
  (bind _returnvalue_3 (Utilities|Enum|Equal(Enum) Winner "NewEnumerator0"))
  (bind _asbp_match_player_state (Utilities|Casting|CastToBP_MatchPlayerState (Variables|/Script/Engine.Controller|GetPlayerState _returnvalue)))
  (bind _returnvalue_4 (UserInterface|CreateWidget "/Game/ProjectAmulet/UI/Menu/Widgets/Widget_Victory.Widget_Victory_C" _returnvalue))
  ;[1 1 1] Is human
  (if (Utilities|Enum|Equal(Enum) (Variables|/Game/ProjectAmulet/Maps/BP_MatchPlayerState.BP_MatchPlayerState_C|GetTeam _asbp_match_player_state) "NewEnumerator0")
    ;[1 1 1] Did you win?
    (if _returnvalue_3
      ;[1 1 1] Human Victory
      (Default|SetImage _returnvalue_4 "/Game/ProjectAmulet/Art/VictoryDefeat/Aliens/Victory_V1__Glitched_3_notext.Victory_V1__Glitched_3_notext" "/Game/ProjectAmulet/Art/VictoryDefeat/Aliens/Backbutton_5_victory.Backbutton_5_victory")
      (else
        ;[1 1 1] Human Defeat
        (Default|SetImage _returnvalue_4 "/Game/ProjectAmulet/Art/VictoryDefeat/Aliens/Defeat_V1_1_Glitched_2_redbg_notext.Defeat_V1_1_Glitched_2_redbg_notext" "/Game/ProjectAmulet/Art/VictoryDefeat/Aliens/Backbutton_defeat.Backbutton_defeat")))
    (elif _returnvalue_3
      ;[1 1 1] Alien Victory
      (Default|SetImage _returnvalue_4 "/Game/ProjectAmulet/Art/VictoryDefeat/Aliens/Victory_V1_Glitched_JMC.Victory_V1_Glitched_JMC" "/Game/ProjectAmulet/Art/VictoryDefeat/Aliens/Backbutton_5_victory.Backbutton_5_victory")
      (else
        ;[1 1 1] Alien Defeat
        (Default|SetImage _returnvalue_4 "/Game/ProjectAmulet/Art/VictoryDefeat/Aliens/Defeat_V1_1_Glitched_2_redbg.Defeat_V1_1_Glitched_2_redbg" "/Game/ProjectAmulet/Art/VictoryDefeat/Aliens/Backbutton_defeat.Backbutton_defeat"))))
  ;[1 1 1] Input UI Only, Players can't move anymore, has to click return to main menu
  (UserInterface|Viewport|AddtoViewport _returnvalue_4 0)
  (Input|SetInputModeUIOnly _returnvalue_2 _returnvalue_4 "DoNotLock")
  (Variables|/Script/Engine.PlayerController|SetbShowMouseCursor _returnvalue_2 true))

(fn VictoryCheck
  (Utilities|Time|ClearandInvalidateTimerbyHandle (Variables|Round|GetTimer))
  (if (== (Variables|Score|GetAlphaWins) 2)
    (CallFunction|MatchEnd "NewEnumerator0")
    (elif (== (Variables|Score|GetBravoWins) 2)
      (CallFunction|MatchEnd "NewEnumerator1")
      (else
        (CallFunction|IncrementRound)))))

(fn ResetAmuletSystem
  (bind _outactors (Actor|GetAllActorsOfClass "/Game/ProjectAmulet/GameMode/EnvironmentBPs/AmuletSpawnLocation.AmuletSpawnLocation_C"))
  (bind _output_get (Variables|Default|SetAmuletLocations _outactors))
  (for _array_element _output_get
    (Default|ResetAmuletLocation _array_element "Visible")))

(fn SpawnRoundScreen
  (bind _currentround (Variables|Round|GetCurrentRound))
  (Development|PrintString "Started Round")
  (bind _returnvalue (UserInterface|CreateWidget "/Game/ProjectAmulet/UI/HUD/WIdget_RoundScreen.WIdget_RoundScreen_C" (Game|GetPlayerController 0)))
  (Default|SetRoundImage _returnvalue)
  (if (== _currentround 2)
    (Default|SetRoundText _returnvalue "OverTime")
    (else
      (Default|SetRoundText _returnvalue (Utilities|String|Append "Round:" (Utilities|String|ToString(Integer) (+ _currentround 1))))))
  (Class|UserWidget|PlayAnimationForward _returnvalue (Variables|/Game/ProjectAmulet/UI/HUD/WIdget_RoundScreen.WIdget_RoundScreen_C|GetRound1_Fade _returnvalue) 1.0 false)
  (UserInterface|Viewport|AddtoViewport _returnvalue 0))

(fn ShouldFreeze
  (params (Team :type BP_ETeam%20Enum :default "NewEnumerator0"))
  (return (Utilities|Enum|Equal(Enum) Team (Variables|Round|GetAttackingTeam))))

(fn OnRepAttackingTeam
  (bind _asbp_gameplay_pc (Utilities|Casting|CastToBP_GameplayPC (Game|GetPlayerController 0)))
  (Default|CheckFreeze _asbp_gameplay_pc true))