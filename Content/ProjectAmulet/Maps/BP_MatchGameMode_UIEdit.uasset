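; Match game mode for a round-based, two-team attack/defend game built around amulet spawn locations.
; A pre-round freezes Alpha and opens amulet spawns, then the timed round unfreezes them, locks spawns and deducts defense costs, with timers run by BP_MatchGameState.
; ChoosePlayerStart builds team rosters from tagged PlayerStarts, and respawns pick random team spawns by attacking side.
; WinCon results and life losses update the GameState and reset player positions.
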(event Custom|ResetRound
  (CallFunction|WinReset))

(event EventBeginPlay
  (CallFunction|StartPreRound))

(fn ConstructionScript)

(fn EarnPointAttackers
  (bind _asbp_match_game_state (Utilities|Casting|CastToBP_MatchGameState (Game|GetGameState)))
  (Default|EarnAttackerPoint _asbp_match_game_state)
  (CallFunction|EndRound))

(fn EarnPointDefenders
  (bind _asbp_match_game_state (Utilities|Casting|CastToBP_MatchGameState (Game|GetGameState)))
  (Default|EarnDefenderPoint _asbp_match_game_state)
  (CallFunction|EndRound))

(fn EndRound
  (CallFunction|ResetPlayerLocations))

(fn AlphaLoseLife
  (bind _asbp_match_game_state (Utilities|Casting|CastToBP_MatchGameState (Game|GetGameState)))
  (bind _iseliminated (Default|AlphaLoseLife _asbp_match_game_state))
  (if _iseliminated
    (CallFunction|EndRound)))

(fn BravoLoseLife
  (bind _asbp_match_game_state (Utilities|Casting|CastToBP_MatchGameState (Game|GetGameState)))
  (bind _iseliminated (Default|BravoLoseLife _asbp_match_game_state))
  (if _iseliminated
    (CallFunction|EndRound)))

(fn CheckAmuletLocation
  ;[1 1 1] Get Active Spawn Location and check point cost
  (bind _outactors (Actor|GetAllActorsOfClass "/Game/ProjectAmulet/GameMode/EnvironmentBPs/AmuletSpawnLocation.AmuletSpawnLocation_C"))
  (bind _output_get (LocalVariables|SetSpawnLocations _outactors))
  (for _array_element _output_get
    (Variables|/Game/ProjectAmulet/GameMode/EnvironmentBPs/AmuletSpawnLocation.AmuletSpawnLocation_C|SetSpawnLocationsActive? _array_element false)
    (if (Variables|/Game/ProjectAmulet/GameMode/EnvironmentBPs/AmuletSpawnLocation.AmuletSpawnLocation_C|GetAmuletSpawned? _array_element)
      (Variables|Default|SetDefensePoints (- (Variables|Default|GetDefensePoints) (Variables|/Game/ProjectAmulet/GameMode/EnvironmentBPs/AmuletSpawnLocation.AmuletSpawnLocation_C|GetDefenseCost _array_element))))))

(fn ActivateSpawnLocations
  (bind _outactors (Actor|GetAllActorsOfClass "/Game/ProjectAmulet/GameMode/EnvironmentBPs/AmuletSpawnLocation.AmuletSpawnLocation_C"))
  (bind _output_get (LocalVariables|SetSpawnLocations _outactors))
  (for _array_element _output_get
    (Variables|/Game/ProjectAmulet/GameMode/EnvironmentBPs/AmuletSpawnLocation.AmuletSpawnLocation_C|SetSpawnLocationsActive? _array_element true)))

(fn WinReset
  (bind _returnvalue (Actor|GetActorOfClass "/Game/ProjectAmulet/GameMode/EnvironmentBPs/WinCon.WinCon_C"))
  (if (Variables|/Game/ProjectAmulet/GameMode/EnvironmentBPs/WinCon.WinCon_C|GetWin? _returnvalue)
    (Scoring|EarnPointAttackers)
    (else
      (Scoring|EarnPointDefenders)))
  (CallFunction|EndRound)
  (Development|PrintString "reset level"))

(fn FreezeAttackers
  (Development|PrintString "Froze Attackers")
  (for _array_element (Variables|Default|GetAlphaTeam)
    (bind _asbp_gameplay_pc (Utilities|Casting|CastToBP_GameplayPC _array_element))
    (Input|SetIgnoreMoveInput _asbp_gameplay_pc true)))

(fn UnFreezeAttackers
  (Development|PrintString "UnFroze Attackers")
  (for _array_element (Variables|Default|GetAlphaTeam)
    (bind _asbp_gameplay_pc (Utilities|Casting|CastToBP_GameplayPC _array_element))
    (Input|SetIgnoreMoveInput _asbp_gameplay_pc false)))

(fn SetMatchTime
  (params (Time :type Float%20%28single-precision%29))
  (Variables|Default|SetMatchTime Time))

(fn StartPreRound
  ;[1 1 1] Starts the preperation phase of the round
  (CallFunction|FreezeAttackers)
  (CallFunction|ActivateSpawnLocations)
  (Default|StartPreRoundTimer (Variables|Default|GetGameStateRef) (Variables|Default|GetPrePhaseTime) "StartRound"))

(fn StartRound
  ;[1 1 1] Starts the main round
  (CallFunction|UnFreezeAttackers)
  (CallFunction|CheckAmuletLocation)
  (Default|StartRoundTimer (Variables|Default|GetGameStateRef) (Variables|Default|GetMatchTime)))

(fn ChoosePlayerStart
  (params (Player :type Controller%20Object%20Reference))
  (if (Variables|Default|GetFirstPlayerSpawned)
    _
    (else
      (CallFunction|InitSpawnPoints)))
  (bind _assteam_game_instance (Utilities|Casting|CastToSteamGameInstance (Game|GetGameInstance)))
  (if (== (Variables|/Game/ProjectAmulet/Core/Networking/SteamGameInstance.SteamGameInstance_C|GetNumPlayers _assteam_game_instance) (Variables|Default|GetPlayersSpawned))
    (bind _playerstart (CallFunction|RespawnPlayer Player))
    (LocalVariables|SetNewSpawnLocation _playerstart)
    (else
      (bind _returnvalue (CallFunction|InitTeams Player))
      (Variables|Default|SetPlayersSpawned (+ (Variables|Default|GetPlayersSpawned) 1))
      (LocalVariables|SetNewSpawnLocation _returnvalue)))
  (return (LocalVariables|GetNewSpawnLocation)))

(fn InitSpawnPoints
  (CallFunction|InitGameState)
  (bind _outactors (Actor|GetAllActorsOfClass "/Script/Engine.PlayerStart"))
  (bind _output_get (Variables|Default|SetSpawnPoints _outactors))
  (Variables|Default|SetPlayerStarts _output_get)
  (Variables|Default|SetFirstPlayerSpawned true))

(fn InitGameState
  (bind _asbp_match_game_state (Utilities|Casting|CastToBP_MatchGameState (Game|GetGameState)))
  (Variables|Default|SetGameStateRef _asbp_match_game_state))

(fn InitTeams
  (params (Player :type Controller%20Object%20Reference))
  (bind _playerstate (Variables|/Script/Engine.Controller|GetPlayerState Player))
  (for _array_element (Variables|Default|GetPlayerStarts)
    (switch name (Variables|/Script/Engine.PlayerStart|GetPlayerStartTag _array_element)
      (:Alpha
        (bind _asbp_match_player_state (Utilities|Casting|CastToBP_MatchPlayerState _playerstate))
        (if (Utilities|Enum|Equal(Enum) (Variables|/Game/ProjectAmulet/Maps/BP_MatchPlayerState.BP_MatchPlayerState_C|GetTeam _asbp_match_player_state) "NewEnumerator0")
          (Utilities|Array|AddUnique (Variables|Default|GetAlphaSpawns) _array_element)
          (bind _asbp_gameplay_pc (Utilities|Casting|CastToBP_GameplayPC Player))
          (Utilities|Array|AddUnique (Variables|Default|GetAlphaTeam) _asbp_gameplay_pc)
          (LocalVariables|SetNewSpawnLocation _array_element :!label _label)))
      (:Bravo
        (bind _asbp_match_player_state_2 (Utilities|Casting|CastToBP_MatchPlayerState _playerstate))
        (if (Utilities|Enum|Equal(Enum) (Variables|/Game/ProjectAmulet/Maps/BP_MatchPlayerState.BP_MatchPlayerState_C|GetTeam _asbp_match_player_state_2) "NewEnumerator1")
          (Utilities|Array|AddUnique (Variables|Default|GetBravoSpawns) _array_element)
          (bind _asbp_gameplay_pc_2 (Utilities|Casting|CastToBP_GameplayPC Player))
          (Utilities|Array|AddUnique (Variables|Default|GetBravoTeam) _asbp_gameplay_pc_2)
          (goto _label)))))
  (Utilities|Array|RemoveItem (Variables|Default|GetPlayerStarts) (LocalVariables|GetNewSpawnLocation))
  (return (LocalVariables|GetNewSpawnLocation)))

(fn RespawnPlayer
  (params (Controller :type Controller%20Object%20Reference))
  (CallFunction|InitGameState)
  (bind _asbp_match_player_state (Utilities|Casting|CastToBP_MatchPlayerState (Variables|/Script/Engine.Controller|GetPlayerState Controller)))
  (if (Utilities|Enum|Equal(Enum) (Variables|/Game/ProjectAmulet/Maps/BP_MatchGameState.BP_MatchGameState_C|GetAttackingTeam (Variables|Default|GetGameStateRef)) (Variables|/Game/ProjectAmulet/Maps/BP_MatchPlayerState.BP_MatchPlayerState_C|GetTeam _asbp_match_player_state))
    (LocalVariables|SetSpawnPos (.OutItem (Utilities|Array|Random (Variables|Default|GetAlphaSpawns))))
    (else
      (LocalVariables|SetSpawnPos (.OutItem (Utilities|Array|Random (Variables|Default|GetBravoSpawns))))))
  (return (LocalVariables|GetSpawnPos)))

(fn OnKill
  (params (Player :type Character%20Object%20Reference))
  (bind _output_get (LocalVariables|SetController (Pawn|GetController Player)))
  (Pawn|UnPossess _output_get)
  (bind _playerstart (CallFunction|RespawnPlayer (LocalVariables|GetController)))
  (Class|GameModeBase|RestartPlayeratPlayerStart (LocalVariables|GetController) _playerstart))

(fn InitPlayerHUD
  (params (Player :type Controller%20Object%20Reference))
  (bind _output_get (LocalVariables|SetConnectedPlayer Player))
  (bind _asbp_gameplay_pc (Utilities|Casting|CastToBP_GameplayPC _output_get))
  (Default|InitialSetup _asbp_gameplay_pc))

(fn ResetPlayerLocations
  (for (_array_element _array_index) (Variables|Default|GetAlphaTeam)
    (bind _asbp_gameplay_pc (Utilities|Casting|CastToBP_GameplayPC _array_element))
    (Default|ResetPlayerLocation _asbp_gameplay_pc (Transformation|GetActorLocation (Utilities|Array|Get(acopy) (Variables|Default|GetAlphaSpawns) _array_index))))
  (for (_array_element_2 _array_index_2) (Variables|Default|GetBravoTeam)
    (bind _asbp_gameplay_pc_2 (Utilities|Casting|CastToBP_GameplayPC _array_element_2))
    (Default|ResetPlayerLocation _asbp_gameplay_pc_2 (Transformation|GetActorLocation (Utilities|Array|Get(acopy) (Variables|Default|GetBravoSpawns) _array_index_2)))))