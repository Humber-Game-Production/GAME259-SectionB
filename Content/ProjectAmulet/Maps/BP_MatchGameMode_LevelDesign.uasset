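; Level-design game mode running a round-based attack/defense match around amulet placement.
; Each round enables amulet spawn locations during a timed prep phase, then disables them and deducts occupied locations' costs from defense points as the attack begins.
; Timeouts score for defenders; attacker points or team life losses can also end rounds.
; BP_MatchGameState holds scores, lives and the displayed countdown, and its round-reset event triggers each StartRound.
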(event Custom|StartAttackPhase
  ;[1 1 1] Starts the main round
  (CallFunction|CheckAmuletLocation)
  (Variables|Default|SetbIsAttackPhase true)
  (bind _returnvalue (Utilities|Time|SetTimerbyEvent (delegate Custom|RoundTimeUp) (Variables|Default|GetMatchTime)))
  (Variables|Default|SetMatchTimer _returnvalue)
  (Default|CallAttackPhaseStarted))

(event Custom|RoundTimeUp
  ;[1 1 1] Resolves the round ending by time
  (Scoring|EarnPointDefenders))

(event Custom|StartRound
  ;[1 1 1] Starts the preperation phase of the round
  (CallFunction|ActivateAmuletSpawnLocations)
  (Variables|Default|SetbIsAttackPhase false)
  (bind _returnvalue (Utilities|Time|SetTimerbyEvent (delegate Custom|StartAttackPhase) (Variables|Default|GetPrePhaseTime)))
  (Variables|Default|SetPrePhaseTimer _returnvalue)
  (Default|CallRoundReset))

(event EventBeginPlay
  (bind _asbp_match_game_state (Utilities|Casting|CastToBP_MatchGameState (Game|GetGameState)))
  (EventDispatchers|BindEventtoRoundReset _asbp_match_game_state (delegate Custom|StartRound))
  (Default|IncrementRound _asbp_match_game_state (Variables|Default|GetHalftimeRound) (Variables|Default|GetFinalRound)))

(event EventTick
  (params (DeltaSeconds :type Float%20%28single-precision%29))
  (if (Variables|Default|GetbIsAttackPhase)
    (bind _asbp_match_game_state (Utilities|Casting|CastToBP_MatchGameState (Game|GetGameState)))
    (Default|SetRemainingTime _asbp_match_game_state (Utilities|Time|GetTimerRemainingTimebyHandle (Variables|Default|GetMatchTimer)))
    (else
      (bind _asbp_match_game_state_2 (Utilities|Casting|CastToBP_MatchGameState (Game|GetGameState)))
      (Default|SetRemainingTime _asbp_match_game_state_2 (Utilities|Time|GetTimerRemainingTimebyHandle (Variables|Default|GetPrePhaseTimer))))))

(fn ConstructionScript)

(fn EarnPointAttackers
  (bind _asbp_match_game_state (Utilities|Casting|CastToBP_MatchGameState (Game|GetGameState)))
  (Default|EarnAttackerPoint _asbp_match_game_state)
  (CallFunction|EndRound))

(fn EarnPointDefenders
  (bind _asbp_match_game_state (Utilities|Casting|CastToBP_MatchGameState (Game|GetGameState)))
  (Default|EarnDefenderPoint _asbp_match_game_state)
  (CallFunction|EndRound))

(fn EndRound
  (Variables|Default|SetbIsAttackPhase false)
  (Utilities|Time|PauseTimerbyHandle (Variables|Default|GetPrePhaseTimer))
  (Utilities|Time|PauseTimerbyHandle (Variables|Default|GetMatchTimer))
  (bind _asbp_match_game_state (Utilities|Casting|CastToBP_MatchGameState (Game|GetGameState)))
  (Default|IncrementRound _asbp_match_game_state (Variables|Default|GetHalftimeRound) (Variables|Default|GetFinalRound)))

(fn AlphaLoseLife
  (bind _asbp_match_game_state (Utilities|Casting|CastToBP_MatchGameState (Game|GetGameState)))
  (bind _iseliminated (Default|AlphaLoseLife _asbp_match_game_state))
  (if _iseliminated
    (CallFunction|EndRound)))

(fn BravoLoseLife
  (bind _asbp_match_game_state (Utilities|Casting|CastToBP_MatchGameState (Game|GetGameState)))
  (bind _iseliminated (Default|BravoLoseLife _asbp_match_game_state))
  (if _iseliminated
    (CallFunction|EndRound)))

(fn CheckAmuletLocation
  ;[1 1 1] Get Active Spawn Location and check point cost
  (bind _outactors (Actor|GetAllActorsOfClass "/Game/ProjectAmulet/GameMode/EnvironmentBPs/AmuletSpawnLocation_LevelDesignEdit.AmuletSpawnLocation_LevelDesignEdit_C"))
  (bind _output_get (LocalVariables|SetSpawnLocations _outactors))
  (for _array_element _output_get
    (Variables|/Game/ProjectAmulet/GameMode/EnvironmentBPs/AmuletSpawnLocation_LevelDesignEdit.AmuletSpawnLocation_LevelDesignEdit_C|SetSpawnLocationsActive? _array_element false)
    (if (Variables|/Game/ProjectAmulet/GameMode/EnvironmentBPs/AmuletSpawnLocation_LevelDesignEdit.AmuletSpawnLocation_LevelDesignEdit_C|GetAmuletSpawned? _array_element)
      (Variables|Default|SetDefensePoints (- (Variables|Default|GetDefensePoints) (Variables|/Game/ProjectAmulet/GameMode/EnvironmentBPs/AmuletSpawnLocation_LevelDesignEdit.AmuletSpawnLocation_LevelDesignEdit_C|GetDefenseCost _array_element))))))

(fn ActivateAmuletSpawnLocations
  (bind _outactors (Actor|GetAllActorsOfClass "/Game/ProjectAmulet/GameMode/EnvironmentBPs/AmuletSpawnLocation_LevelDesignEdit.AmuletSpawnLocation_LevelDesignEdit_C"))
  (bind _output_get (LocalVariables|SetSpawnLocations _outactors))
  (for _array_element _output_get
    (Variables|/Game/ProjectAmulet/GameMode/EnvironmentBPs/AmuletSpawnLocation_LevelDesignEdit.AmuletSpawnLocation_LevelDesignEdit_C|SetSpawnLocationsActive? _array_element true)))