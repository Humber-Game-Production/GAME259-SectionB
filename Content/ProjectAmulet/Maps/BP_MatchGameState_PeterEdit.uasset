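; Match game state for a two-team attack/defend mode, tracking round wins, team lives, remaining time and a spendable amulet point pool.
; State setters fire events that relay to dispatchers for timer, lives, score, points, round reset and match end.
; A team running out of lives scores for its opponent.
; IncrementRound swaps attackers and refills points at halftime multiples, the only case where the round counter advances.
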(event Custom|Timers
  ;[1 1 1] Event Dispatcher events
  (Default|CallUpdateTimers))

(event Custom|ScoreUpdate
  ;[1 1 1] Event Dispatcher events
  (Default|CallUpdateScore))

(event Custom|AlphaLifeCount
  ;[1 1 1] Event Dispatcher events
  (Default|CallUpdateAlphaLives))

(event Custom|BravoLifeCount
  ;[1 1 1] Event Dispatcher events
  (Default|CallUpdateBravoLives))

(event Custom|MatchEnd
  ;[1 1 1] Event Dispatcher events
  (Default|CallEndOfMatch))

(event Custom|ResetRound
  ;[1 1 1] Event Dispatcher events
  (Default|CallRoundReset))

(event Custom|AmuletPoints
  ;[1 1 1] Event Dispatcher events
  (Default|CallUpdateAmuletPoints))

(event EventBeginPlay)

(event EventTick
  (params (DeltaSeconds :type Float%20%28single-precision%29)))

(fn ConstructionScript)

(fn EarnAttackerPoint
  (switch Utilities|FlowControl|Switch|SwitchonBP_ETeam (Variables|Round|GetAttackingTeam)
    (:NewEnumerator0
      (CallFunction|AddScore true))
    (:NewEnumerator1
      (CallFunction|AddScore false))))

(fn EarnDefenderPoint
  (switch Utilities|FlowControl|Switch|SwitchonBP_ETeam (Variables|Round|GetAttackingTeam)
    (:NewEnumerator0
      (CallFunction|AddScore false))
    (:NewEnumerator1
      (CallFunction|AddScore true))))

(fn SwapTeams
  (switch Utilities|FlowControl|Switch|SwitchonBP_ETeam (Variables|Round|GetAttackingTeam)
    (:NewEnumerator2
      (Variables|Round|SetAttackingTeam "NewEnumerator0" :!label _label))
    (:NewEnumerator0
      (Variables|Round|SetAttackingTeam "NewEnumerator1"))
    (:NewEnumerator1
      (goto _label)))
  (Variables|Round|SetCurrentAmuletPoints (Variables|Round|GetStartingAmuletPoints))
  (CallFunction|AmuletPoints))

(fn GetRemainingTimeMinSec
  (bind _remainingtime (Variables|Round|GetRemainingTime))
  (bind (_remainder _returnvalue) (Math|Float|Division(WholeandRemainder) _remainingtime 6e+01))
  (return _returnvalue (Math|Float|Truncate _remainder)))

(fn SetRemainingTime
  (params (Time :type Float%20%28single-precision%29))
  (Variables|Round|SetRemainingTime Time)
  (CallFunction|Timers))

(fn AlphaLoseLife
  (bind _alphalives (Variables|Score|GetAlphaLives))
  (bind _returnvalue (== _alphalives 0))
  (Math|Integer|DecrementInt _alphalives
    (:%20%20
      (CallFunction|AlphaLifeCount)
      (if _returnvalue
        (CallFunction|AddScore false))
      (return _returnvalue))))

(fn BravoLoseLife
  (bind _bravolives (Variables|Score|GetBravoLives))
  (bind _returnvalue (== _bravolives 0))
  (Math|Integer|DecrementInt _bravolives
    (:%20%20
      (CallFunction|BravoLifeCount)
      (if _returnvalue
        (CallFunction|AddScore true))
      (return _returnvalue))))

(fn IncrementRound
  (params (Halftime :type Integer) (FinalRound :type Integer))
  (bind _currentround (Variables|Round|GetCurrentRound))
  (if (< _currentround FinalRound)
    (if (== (Math|Integer|%(Integer) _currentround Halftime) 0)
      (CallFunction|SwapTeams)
      (Math|Integer|IncrementInt (Variables|Round|GetCurrentRound)
        (:%20%20
          _)))
    (CallFunction|ResetRound)
    (else
      (CallFunction|MatchEnd))))

(fn UseAmuletPoints
  (params (PointsToUse :type Integer))
  (if (<= PointsToUse (Variables|Round|GetCurrentAmuletPoints))
    (Variables|Round|SetCurrentAmuletPoints (- (Variables|Round|GetCurrentAmuletPoints) PointsToUse))
    (CallFunction|AmuletPoints))
  (return (<= PointsToUse (Variables|Round|GetCurrentAmuletPoints))))

(fn AddScore
  (params (IsAlpha :type Boolean))
  (if IsAlpha
    (Math|Integer|IncrementInt (Variables|Score|GetAlphaWins)
      (:%20%20
        _))
    (else
      (Math|Integer|IncrementInt (Variables|Score|GetBravoWins)
        (:%20%20
          _))))
  (CallFunction|ScoreUpdate))