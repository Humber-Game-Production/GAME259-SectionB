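; Match player state that holds a player's team and health in Project Amulet.
; Health changes are clamped and broadcast to the health bar; at zero it calls the player's death, resets and removes the low-health widget.
; The reset restores full health, strips the owner controller's ability and refreshes its icon.
; CopyProperties carries the team to the new player state, then initializes the health bar and runs the reset.
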(event Custom|ChangeHealth
  (params (Value :type Float%20%28single-precision%29) (Player :type TPC%20Network%20Edit%20Object%20Reference))
  (bind _output_get (Variables|Default|SetcurrentHealth (Math|Float|Clamp(Float) (+ (Variables|Default|GetcurrentHealth) Value) 0.0 (Variables|Default|GetmaxHealth))))
  (Default|CallUpdateHealthBar self)
  (if (== _output_get 0.0)
    (Default|CallDeath Player)
    (CallFunction|RespawnUpdate)
    (Widget|RemovefromParent (Variables|Default|GetlowHealthBarWidget))))

(event Custom|SetTeam
  (params (Team :type BP_ETeam%20Enum :default "NewEnumerator2"))
  (Variables|Default|SetTeam Team))

(event Custom|TryChangeTeam
  (params (Team :type BP_ETeam%20Enum :default "NewEnumerator2"))
  (bind _output_get (Variables|Default|SetTeam Team))
  (CallFunction|SetTeam _output_get))

(event Custom|RespawnUpdate
  (Variables|Default|SetcurrentHealth (Variables|Default|GetmaxHealth))
  (Default|CallUpdateHealthBar)
  (bind _astpc_network_edit (Utilities|Casting|CastToTPC_NetworkEdit (Components|GetOwner)))
  (Default|RemoveAbility _astpc_network_edit)
  (Default|CallInitalizeAbilityIcon))

(event EventCopyProperties
  (params (NewPlayerState :type Player%20State%20Object%20Reference))
  (bind _asbp_match_player_state (Utilities|Casting|CastToBP_MatchPlayerState NewPlayerState))
  (Variables|BP_MatchPlayerState_C|SetTeam _asbp_match_player_state (Variables|Default|GetTeam))
  (Default|CallInitHealthBar)
  (CallFunction|RespawnUpdate))

(fn ConstructionScript)

(fn OnRepCurrentHealth)