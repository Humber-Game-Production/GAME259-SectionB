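; Match game state for a two-team attack/defend amulet mode, tracking lives, wins, rounds, remaining time and amulet points.
; State functions fire event dispatchers for changes, and losing a team's last life scores for the opponent.
; IncrementRound swaps attackers at halftime, refilling amulet points, or ends the match after the final round.
; It also directly creates round-screen and objective widgets, including overtime, choosing objective text by attacking team.
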(event Custom|Timers
  ;[1 1 1] Event Dispatcher events
  (Default|CallUpdateTimers))

(event Custom|ScoreUpdate
  ;[1 1 1] Event Dispatcher events
  (Default|CallUpdateScore))

(event Custom|AlphaLifeCount
  ;[1 1 1] Event Dispatcher events
  (Default|CallUpdateAlphaLives))

(event Custom|BravoLifeCount
  ;[1 1 1] Event Dispatcher events
  (Default|CallUpdateBravoLives))

(event Custom|MatchEnd
  ;[1 1 1] Event Dispatcher events
  (Default|CallEndOfMatch))

(event Custom|ResetRound
  ;[1 1 1] Event Dispatcher events
  (Default|CallRoundReset))

(event Custom|AmuletPoints
  ;[1 1 1] Event Dispatcher events
  (Default|CallUpdateAmuletPoints))

(event EventBeginPlay)

(event EventTick
  (params (DeltaSeconds :type Float%20%28single-precision%29)))

(fn ConstructionScript)

(fn EarnAttackerPoint
  (switch Utilities|FlowControl|Switch|SwitchonBP_ETeam (Variables|Round|GetAttackingTeam)
    (:NewEnumerator0
      (CallFunction|AddScore true))
    (:NewEnumerator1
      (CallFunction|AddScore false))))

(fn EarnDefenderPoint
  (switch Utilities|FlowControl|Switch|SwitchonBP_ETeam (Variables|Round|GetAttackingTeam)
    (:NewEnumerator0
      (CallFunction|AddScore false))
    (:NewEnumerator1
      (CallFunction|AddScore true))))

(fn SwapTeams
  (switch Utilities|FlowControl|Switch|SwitchonBP_ETeam (Variables|Round|GetAttackingTeam)
    (:NewEnumerator2
      (Variables|Round|SetAttackingTeam "NewEnumerator0" :!label _label))
    (:NewEnumerator0
      (Variables|Round|SetAttackingTeam "NewEnumerator1"))
    (:NewEnumerator1
      (goto _label)))
  (Variables|Round|SetCurrentAmuletPoints (Variables|Round|GetStartingAmuletPoints))
  (CallFunction|AmuletPoints))

(fn GetRemainingTimeMinSec
  (bind _remainingtime (Variables|Round|GetRemainingTime))
  (bind (_remainder _returnvalue) (Math|Float|Division(WholeandRemainder) _remainingtime 6e+01))
  (return _returnvalue (Math|Float|Truncate _remainder)))

(fn SetRemainingTime
  (params (Time :type Float%20%28single-precision%29))
  (Variables|Round|SetRemainingTime Time)
  (CallFunction|Timers))

(fn AlphaLoseLife
  (bind _alphalives (Variables|Score|GetAlphaLives))
  (bind _returnvalue (== _alphalives 0))
  (Math|Integer|DecrementInt _alphalives
    (:%20%20
      (CallFunction|AlphaLifeCount)
      (if _returnvalue
        (CallFunction|AddScore false))
      (return _returnvalue))))

(fn BravoLoseLife
  (bind _bravolives (Variables|Score|GetBravoLives))
  (bind _returnvalue (== _bravolives 0))
  (Math|Integer|DecrementInt _bravolives
    (:%20%20
      (CallFunction|BravoLifeCount)
      (if _returnvalue
        (CallFunction|AddScore true))
      (return _returnvalue))))

(fn IncrementRound
  (params (Halftime :type Integer) (FinalRound :type Integer))
  (bind _currentround (Variables|Round|GetCurrentRound))
  (if (< _currentround FinalRound)
    (if (== (Math|Integer|%(Integer) _currentround Halftime) 0)
      (CallFunction|SwapTeams)
      (Math|Integer|IncrementInt (Variables|Round|GetCurrentRound)
        (:%20%20
          _)))
    (CallFunction|ResetRound)
    ;[1 1 1] Set Objective Message Depending on Team Alpha or Bravo
    ;;[1 1 1] Remove widgets after round resets then do if check to add appropriate objective/round widget
    (Widget|RemovefromParent (stale _returnvalue))
    (if (Utilities|Enum|Equal(Enum) (Variables|Round|GetAttackingTeam) "NewEnumerator0")
      (bind _returnvalue (UserInterface|CreateWidget "/Game/ProjectAmulet/UI/HUD/Widget_Objective.Widget_Objective_C" 0 "Retrieve the amulet!"))
      (UserInterface|Viewport|AddtoViewport _returnvalue 0)
      ;[1 1 1] Add Round Screen Widgets Depending on Current Round
      ;;[1 1 1] Round 1
      (if (== (Variables|Round|GetCurrentRound) 0) :!label _label
        (bind _returnvalue_2 (UserInterface|CreateWidget "/Game/ProjectAmulet/UI/HUD/WIdget_RoundScreen.WIdget_RoundScreen_C"))
        (Class|UserWidget|PlayAnimationForward _returnvalue_2 (Variables|/Game/ProjectAmulet/UI/HUD/WIdget_RoundScreen.WIdget_RoundScreen_C|GetRound1_Fade _returnvalue_2) 1.0 false)
        (UserInterface|Viewport|AddtoViewport _returnvalue_2 0)
        (else
          ;;[1 1 1] Round 2
          (if (== (Variables|Round|GetCurrentRound) 1)
            (bind _returnvalue_3 (UserInterface|CreateWidget "/Game/ProjectAmulet/UI/HUD/WIdget_RoundScreen.WIdget_RoundScreen_C"))
            (Class|UserWidget|PlayAnimationForward _returnvalue_3 (Variables|/Game/ProjectAmulet/UI/HUD/WIdget_RoundScreen.WIdget_RoundScreen_C|GetRound2_Fade _returnvalue_3) 1.0 false)
            (UserInterface|Viewport|AddtoViewport _returnvalue_3 0)
            (else
              ;;[1 1 1] Overtime
              (if (== (Variables|Round|GetCurrentRound) 2)
                (bind _returnvalue_4 (UserInterface|CreateWidget "/Game/ProjectAmulet/UI/HUD/WIdget_RoundScreen.WIdget_RoundScreen_C"))
                (Class|UserWidget|PlayAnimationForward _returnvalue_4 (Variables|/Game/ProjectAmulet/UI/HUD/WIdget_RoundScreen.WIdget_RoundScreen_C|GetOvertime_Fade _returnvalue_4) 1.0 false)
                (UserInterface|Viewport|AddtoViewport _returnvalue_4 0)
                ;[1 1 1] If overtime, add overtime objective message
                ;;[1 1 1] Remove alpha/beta objective message as both teams will have same message in overtime mode
                (Widget|RemovefromParent _returnvalue)
                ;;[1 1 1] Set the overtime objective message
                (bind _returnvalue_5 (UserInterface|CreateWidget "/Game/ProjectAmulet/UI/HUD/Widget_Objective.Widget_Objective_C" 0 "Eliminate the enemy team!"))
                (UserInterface|Viewport|AddtoViewport _returnvalue_5 0))))))
      (elif (Utilities|Enum|Equal(Enum) (Variables|Round|GetAttackingTeam) "NewEnumerator1")
        (bind _returnvalue_6 (UserInterface|CreateWidget "/Game/ProjectAmulet/UI/HUD/Widget_Objective.Widget_Objective_C" 0 "Protect the amulet!"))
        (UserInterface|Viewport|AddtoViewport _returnvalue_6 0)
        (goto _label)))
    (else
      (CallFunction|MatchEnd))))

(fn UseAmuletPoints
  (params (PointsToUse :type Integer))
  (if (<= PointsToUse (Variables|Round|GetCurrentAmuletPoints))
    (Variables|Round|SetCurrentAmuletPoints (- (Variables|Round|GetCurrentAmuletPoints) PointsToUse))
    (CallFunction|AmuletPoints))
  (return (<= PointsToUse (Variables|Round|GetCurrentAmuletPoints))))

(fn AddScore
  (params (IsAlpha :type Boolean))
  (if IsAlpha
    (Math|Integer|IncrementInt (Variables|Score|GetAlphaWins)
      (:%20%20
        _))
    (else
      (Math|Integer|IncrementInt (Variables|Score|GetBravoWins)
        (:%20%20
          _))))
  (CallFunction|ScoreUpdate))