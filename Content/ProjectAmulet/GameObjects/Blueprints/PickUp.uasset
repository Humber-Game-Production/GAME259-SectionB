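; Ability pickup actor that grants its configured Ability to an overlapping TPC character.
; BeginPlay sets the mesh, scale and any material or rotation for rocket, wall, shield or ambrosia, then bobs it through a looping MoveComponentTo and FlipFlop.
; Overlap, bound on every Tick, adds the ability and hides the actor until a 15-second timer shows it again.
; Hiding leaves collision unchanged.
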(event Custom|Give%20Ability
  (params (OverlappedActor :type Actor%20Object%20Reference) (OtherActor :type Actor%20Object%20Reference))
  (bind _astpc (Utilities|Casting|CastToTPC OtherActor))
  (Default|AddAbility _astpc (Variables|Default|GetAbility))
  ;[1 1 1] Respawn Iteam
  (Rendering|SetActorHiddenInGame self true)
  (Utilities|Time|SetTimerbyEvent (delegate Custom|ReEnable) 15.0))

(event Custom|ReEnable
  ;[1 1 1] Respawn Iteam
  (Rendering|SetActorHiddenInGame false))

(event EventTick
  (params (DeltaSeconds :type Float%20%28single-precision%29))
  (Collision|BindEventtoOnActorBeginOverlap (delegate Custom|Give%20Ability)))

(event EventBeginPlay
  (bind _abilityweapon (Variables|Default|GetAbilityWeapon))
  (bind _abilityweapon_2 (Variables|Default|GetAbilityWeapon))
  (bind _abilityweapon_3 (Variables|Default|GetAbilityWeapon))
  (bind _abilityweapon_4 (Variables|Default|GetAbilityWeapon))
  (bind _abilityweapon_5 (Variables|Default|GetAbilityWeapon))
  (bind _relativelocation (Variables|/Script/Engine.SceneComponent|GetRelativeLocation _abilityweapon_5))
  (if (== (Variables|Default|GetAbility) "/Script/GAME259Prod_SecB.AbilityRocket")
    (Components|StaticMesh|SetStaticMesh _abilityweapon "/Game/ProjectAmulet/Maps/Assets/StaticMesh/Weapons/Bazookatube_Weapon_SM.Bazookatube_Weapon_SM")
    (Transformation|SetWorldScale3D _abilityweapon "1.500000,1.500000,1.300000")
    (Components|MoveComponentTo _abilityweapon_5 (Math|Vector|SelectVector (+ _relativelocation "0, 0,30.000000") (- _relativelocation "0, 0,30.000000") (Variables|Default|GetReset)) (Variables|/Script/Engine.SceneComponent|GetRelativeRotation _abilityweapon_5) true true 2.0 false :!label _label)
    (Utilities|FlowControl|FlipFlop
      (:A
        (Variables|Default|SetReset false)
        (goto _label))
      (:B
        (Variables|Default|SetReset true)
        (goto _label)))
    (elif (== (Variables|Default|GetAbility) "/Script/GAME259Prod_SecB.AbilityWall")
      (Components|StaticMesh|SetStaticMesh _abilityweapon_4 "/Game/ProjectAmulet/Maps/Assets/StaticMesh/Weapons/DWC_Deployable_Shield.DWC_Deployable_Shield")
      (Transformation|SetWorldScale3D _abilityweapon_4 "0.400000,0.400000,0.400000")
      (goto _label)
      (elif (== (Variables|Default|GetAbility) "/Script/GAME259Prod_SecB.AbilityShield")
        (Components|StaticMesh|SetStaticMesh _abilityweapon_2 "/Game/StarterContent/Props/MaterialSphere.MaterialSphere")
        (Rendering|Material|SetMaterial _abilityweapon_2 0 "/Game/ProjectAmulet/Maps/Assets/Materials/Effects/Energy_Shield/M_Shield_001_ARA.M_Shield_001_ARA")
        (Transformation|SetWorldScale3D _abilityweapon_2 "0.800000,0.800000,0.800000")
        (goto _label)
        (elif (== (Variables|Default|GetAbility) "/Script/GAME259Prod_SecB.AbilityAmbrosia")
          (Components|StaticMesh|SetStaticMesh _abilityweapon_3 "/Game/StarterContent/Shapes/AmuletPlane.AmuletPlane")
          (Rendering|Material|SetMaterial _abilityweapon_3 0 "/Game/ProjectAmulet/Art/Materials/M_AmbrosiaBillboard.M_AmbrosiaBillboard")
          (Transformation|SetWorldScale3D _abilityweapon_3 "2.000000,2.500000,2.000000")
          (Transformation|SetWorldRotation _abilityweapon_3 "0,-90.000000, 0" false false)
          (goto _label))))))

(fn ConstructionScript)