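; Environmental seagull Blueprint that circles around a center point while bobbing up and down.
; Each Tick sets the Rotate component's yaw from game time and RotationSpeed, and offsets DistanceFromCenter by the orbit radius with a sine-driven height.
; The construction script applies the same radius offset so the placement shows in the editor.
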(event EventBeginPlay)

(event EventTick
  (params (DeltaSeconds :type Float%20%28single-precision%29))
  (bind _returnvalue (Utilities|Time|GetGameTimeinSeconds))
  (Transformation|SetRelativeRotation (Variables|Default|Getrotate) (Math|Rotator|MakeRotator 0.0 0.0 (* _returnvalue (Variables|Default|GetRotationSpeed))) false false)
  (Transformation|SetRelativeLocation (Variables|Default|GetdistanceFromCenter) (Math|Vector|MakeVector 0.0 (Variables|Default|GetDistance%20From%20Center) (* (Math|Trig|Sin(Radians) (* _returnvalue (Variables|Default|GetUpDownSpeed))) (Variables|Default|GetUpDownAmount))) false false))

(fn ConstructionScript
  (Transformation|SetRelativeLocation (Variables|Default|GetdistanceFromCenter) (Math|Vector|MakeVector 0.0 (Variables|Default|GetDistance%20From%20Center) 0.0) false false))