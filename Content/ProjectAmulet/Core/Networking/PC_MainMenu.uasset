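; Main menu player controller that loads the local player's Steam profile and online friends list on BeginPlay.
; After a short delay it logs whether the Steam subsystem exists, reads the player name either way, then fetches the avatar asynchronously.
; The profile is saved through game instance interface messages, which also trigger the menu's player info.
; It then fetches friends, requesting avatars for online ones and forwarding each to the game instance.
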(event EventBeginPlay
  (bind _returnvalue (Game|GetGameInstance))
  (Utilities|FlowControl|Delay 0.2)
  (if (Class|AdvancedSessionsLibrary|HasOnlineSubsystem "STEAM")
    (Development|PrintString "Steam Is There")
    (Variables|Default|SetSteamName (Utilities|Text|ToText(String) (Class|AdvancedSessionsLibrary|GetPlayerName self)))
    (else
      (Development|PrintString "Steam Is Not There")
      (Variables|Default|SetSteamName (Utilities|Text|ToText(String) (Class|AdvancedSessionsLibrary|GetPlayerName self)))))
  (bind _returnvalue_2 (Class|AdvancedSteamFriendsLibrary|GetSteamFriendAvatar (Class|AdvancedSessionsLibrary|GetUniqueNetID self) "SteamAvatar_Medium")
    (:OnSuccess
      (bind _structout (Utilities|Struct|SetmembersinS_PlayerInfo (Variables|Default|GetPlayerInfo) (Variables|Default|GetSteamName) _returnvalue_2))
      (bind _returnvalue_3 (Class|BPIGameInstance|SteamGameInstanceRef(Message) _returnvalue))
      (Class|BPIGameInstance|SavePlayerInfo(Message) _returnvalue_3 (Utilities|Struct|MakeS_PlayerInfo (.SteamName (Utilities|Struct|BreakS_PlayerInfo _structout)) (.PlayerStatus (Utilities|Struct|BreakS_PlayerInfo _structout)) (.PlayerImage (Utilities|Struct|BreakS_PlayerInfo _structout))))
      (Class|BPIGameInstance|MainMenuPlayerInfo(Message) _returnvalue)
      (bind _results (|GetandStoreFriendsList (Game|GetPlayerController 0))
        (:OnSuccess
          (for _array_element _results
            (if (Utilities|Struct|BreakBPFriendPresenceInfo (.PresenceInfo (Utilities|Struct|BreakBPFriendInfo _array_element)))
              (bind _returnvalue_4 (Class|AdvancedSteamFriendsLibrary|GetSteamFriendAvatar (.UniqueNetId (Utilities|Struct|BreakBPFriendInfo _array_element)) "SteamAvatar_Medium")
                (:OnSuccess
                  (Class|BPIGameInstance|UpdateFriendList(Message) (Game|GetGameInstance) _array_element _returnvalue_4))))))))))

(fn ConstructionScript)