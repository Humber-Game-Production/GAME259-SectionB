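; Lobby game mode for a Steam multiplayer session that tracks connected players, shares host map settings, handles kicks and starts the match.
; It pushes settings, player info and loading screens to each lobby player controller through interface-style messages.
; Server name and player limit come from the Steam game instance, which receives player count and lobby state updates.
; Launch uses ServerTravel, with both map IDs currently pointing to one placeholder adventure level.
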(event Custom|SpawnPlayer
  (params (Player :type Player%20Controller%20Object%20Reference)))

(event Custom|UpdateServerPlayers
  (params (NumPlayers :type Integer))
  (Development|PrintString (Utilities|String|ToString(Integer) NumPlayers))
  (bind _gameinstance (Class|BPIGameInstance|SteamGameInstanceRef(Message) (Game|GetGameInstance)))
  (Default|ToggleNumPlayers _gameinstance NumPlayers))

(event Custom|HostUpdateGameSettings
  (params (SelectedMapImage :type Texture%202D%20Object%20Reference) (SelectedMapName :type Text) (SelectedMapTime :type Text) (SelectedMapID :type Integer))
  ;[1 1 1] Updates clients to update when server makes changes
  (Variables|Default|SetSelectedMapImage SelectedMapImage)
  (Variables|Default|SetSelectedMapName SelectedMapName)
  (Variables|Default|SetSelectedMapTime SelectedMapTime)
  (Variables|Default|SetSelectedMapID SelectedMapID)
  (for _array_element (Variables|Default|GetConnectedPlayers)
    (bind _lobbypc (Class|BPILobbyPlayerController|LobbyPCRef(Message) _array_element))
    (Default|UpdateLobbySettings _lobbypc (Variables|Default|GetSelectedMapImage) (Variables|Default|GetSelectedMapName) (Variables|Default|GetSelectedMapTime))))

(event Custom|PlayerKicked
  (params (PlayerID :type Integer))
  ;[1 1 1] Kicks selected player
  (bind _lobbypc (Class|BPILobbyPlayerController|LobbyPCRef(Message) (Utilities|Array|Get(acopy) (Variables|Default|GetConnectedPlayers) PlayerID)))
  (Default|Kicked _lobbypc))

(event Custom|StartLoadingScreen
  ;[1 1 1] Will show loading screen and launch selected level
  (for _array_element (Variables|Default|GetConnectedPlayers)
    (bind _lobbypc (Class|BPILobbyPlayerController|LobbyPCRef(Message) _array_element))
    (Default|ShowLoadingScreen _lobbypc))
  (CallFunction|LaunchGame))

(event Custom|AddToKickList
  ;[1 1 1] Adds players to kick list
  (bind _lobbypc (Class|BPILobbyPlayerController|LobbyPCRef(Message) (Game|GetPlayerController 0)))
  (Default|AddPlayertoKickWindow _lobbypc))

(event Custom|EveryoneUpdate
  (bind _connectedplayers (Variables|Default|GetConnectedPlayers))
  ;[1 0.6353 0.2816] Updates most information every time someone connects
  (bind _output_get (Variables|Default|SetCurrentPlayers (Utilities|Array|Length (Variables|Default|GetConnectedPlayers))))
  (CallFunction|UpdateServerPlayers _output_get)
  (if (> _output_get 0)
    (Utilities|Array|Clear (Variables|Default|GetConnectedPlayersInfo))
    (for _array_element _connectedplayers
      (bind _lobbypc (Class|BPILobbyPlayerController|LobbyPCRef(Message) _array_element))
      (Utilities|Array|AddUnique (Variables|Default|GetConnectedPlayersInfo) (Variables|/Game/ProjectAmulet/Core/Networking/Lobby/BP_LobbyPC.BP_LobbyPC_C|GetPlayerSettings _lobbypc))
      (Default|UpdateNumberOfPlayers _lobbypc (Variables|Default|GetCurrentPlayers) (Variables|Default|GetMax%20Players)))
    (for _array_element_2 _connectedplayers
      (bind _lobbypc_2 (Class|BPILobbyPlayerController|LobbyPCRef(Message) _array_element_2))
      (Default|AddPlayerInfo _lobbypc_2 (Variables|Default|GetConnectedPlayersInfo))
      (CallFunction|AddtoKickList))))

(event Custom|UpdateInLobby
  (params (InLobby :type Boolean))
  (bind _gameinstance (Class|BPIGameInstance|SteamGameInstanceRef(Message) (Game|GetGameInstance)))
  (Default|ToggleinLobby _gameinstance InLobby))

(event Custom|LaunchGame
  (bind _returnvalue (Game|GetPlayerController 0))
  (switch int (Variables|Default|GetSelectedMapID)
    (:0
      ;[0.1382 0.3607 1] This needs to be changed to location of maps when we have them
      (Development|ExecuteConsoleCommand "ServerTravel L_Adventure_JAA_002" _returnvalue))
    (:1
      (Development|ExecuteConsoleCommand "ServerTravel L_Adventure_JAA_002" _returnvalue))))

(event EventOnLogout
  (params (ExitingController :type Controller%20Object%20Reference))
  (bind _connectedplayers (Variables|Default|GetConnectedPlayers))
  ;[1 1 1] Removes player info when disconnected (if there will be character selection, important work will need to be added here to free up characters)
  (bind (_array_element _array_index) (Utilities|Array|ForEachLoopwithBreak _connectedplayers :!label _label)
    (:LoopBody
      (if (== ExitingController _array_element)
        (goto _label Break)))
    (:Completed
      (Class|BPILobbyPlayerController|LobbyPCRef(Message) (Utilities|Array|Get(acopy) _connectedplayers _array_index))
      (Utilities|Array|RemoveIndex (Variables|Default|GetConnectedPlayers) _array_index)
      (Utilities|Array|RemoveIndex (Variables|Default|GetConnectedPlayersInfo) _array_index)
      (CallFunction|EveryoneUpdate))))

(event EventBeginPlay
  (bind _outactors (Actor|GetAllActorsOfClass "/Script/Engine.PlayerStart"))
  (Variables|Default|SetSpawnPoints _outactors)
  (bind _gameinstance (Class|BPIGameInstance|SteamGameInstanceRef(Message) (Game|GetGameInstance)))
  (Variables|Default|SetServer%20Name (Variables|/Game/ProjectAmulet/Core/Networking/SteamGameInstance.SteamGameInstance_C|GetServerName _gameinstance))
  (Variables|Default|SetMax%20Players (Variables|/Game/ProjectAmulet/Core/Networking/SteamGameInstance.SteamGameInstance_C|GetMaxPlayers _gameinstance)))

(event EventPostLogin
  (params (NewPlayer :type Player%20Controller%20Object%20Reference))
  ;[1 1 1] Initial setup that runs when someone connects
  (bind _output_get (Variables|Default|SetConnectedPlayer NewPlayer))
  (Utilities|Array|AddUnique (Variables|Default|GetConnectedPlayers) _output_get)
  (Utilities|FlowControl|Delay 0.5)
  (bind _lobbypc (Class|BPILobbyPlayerController|LobbyPCRef(Message) (Variables|Default|GetConnectedPlayer)))
  (Default|InitialSetup _lobbypc (Variables|Default|GetServer%20Name) (Variables|Default|GetSelectedMapImage) (Variables|Default|GetSelectedMapName) (Variables|Default|GetSelectedMapTime)))

(fn ConstructionScript)

(fn OnKill
  (params (NewParam :type Character%20Object%20Reference))
  (bind _output_get (LocalVariables|SetController (Pawn|GetController NewParam)))
  (Pawn|UnPossess _output_get)
  (Class|GameModeBase|RestartPlayer (LocalVariables|GetController)))

(fn LobbyGMRef
  (return self))