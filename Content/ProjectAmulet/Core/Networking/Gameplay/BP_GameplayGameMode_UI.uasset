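; Gameplay game mode that handles player spawning, text chat and session teardown on logout.
; It records swapped-in PlayerControllers and relays chat messages to each through interface calls.
; For controllers without a valid pawn, it spawns the selected character at a random PlayerStart and possesses it.
; On logout, it asks the Steam GameInstance to destroy the session for the exiting controller.
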(event Custom|SpawnPlayer
  (params (PlayerController :type Player%20Controller%20Object%20Reference) (SelectedCharacter :type Character%20Class%20Reference))
  ;[1 1 1] Spawns player at random location (will most likely need to change if we are not doing random spawns)
  ; (Also might need to change the passing in of character class to predefined characters if we are not letting players choose their character)
  (bind _outactors (Actor|GetAllActorsOfClass "/Script/Engine.PlayerStart"))
  (Variables|Default|SetSpawnPoints _outactors)
  (Utilities|IsValid (Pawn|GetControlledPawn PlayerController)
    (:Is%20Valid
      (Actor|DestroyActor))
    (:Is%20Not%20Valid
      (bind _returnvalue (Game|SpawnActorfromClass SelectedCharacter (Transformation|GetActorTransform (Utilities|Array|Get(acopy) (Variables|Default|GetSpawnPoints) (Math|Random|RandomIntegerinRange 0 (- (Utilities|Array|Length (Variables|Default|GetSpawnPoints)) 1)))) "Undefined" 0 0))
      (Pawn|Possess PlayerController _returnvalue))))

(event Custom|UpdateChat
  (params (Sender :type Text) (ChatText :type Text))
  (for _array_element (Variables|Default|GetAllPlayerControllers)
    (bind _gameplaypc (Class|BPIGamePlayPC|GameplayPCref(Message) _array_element))
    (Default|UpdateChatWindow _gameplaypc Sender ChatText)))

(event EventOnSwapPlayerControllers
  (params (OldPC :type Player%20Controller%20Object%20Reference) (NewPC :type Player%20Controller%20Object%20Reference))
  (Utilities|Array|Add (Variables|Default|GetAllPlayerControllers) NewPC))

(event EventOnLogout
  (params (ExitingController :type Controller%20Object%20Reference))
  ;[1 1 1] Destroys session on logout
  (bind _gameplaypc (Class|BPIGamePlayPC|GameplayPCref(Message) ExitingController))
  (bind _gameinstance (Class|BPIGameInstance|SteamGameInstanceRef(Message) (Game|GetGameInstance)))
  (Class|BPIGameInstance|DestroySessionCaller(Message) _gameinstance _gameplaypc))

(fn ConstructionScript)

(fn GameplayGMRef
  (return self))