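; BP_GameplayPC is the gameplay player controller, handling HUD creation, compass bearing and respawn hooks.
; Setup events trigger RespawnUpdate on the match player state and add HUD, compass and objective widgets to the viewport.
; Each tick it converts the amulet location into the controlled character's mesh space and broadcasts the negated yaw as the compass bearing.
; ResetPlayerLocation forwards a location to the controlled character's reset.
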(event Custom|InitialSetup
  (bind _asbp_match_player_state (Utilities|Casting|CastToBP_MatchPlayerState (Variables|GetPlayerState)))
  (Default|RespawnUpdate _asbp_match_player_state))

(event Custom|SetupPlayerHud
  ;[1 1 1] Player HUD
  (bind _returnvalue (UserInterface|CreateWidget "/Game/ProjectAmulet/UI/HUD/Widget_PlayerHUD.Widget_PlayerHUD_C" self))
  (UserInterface|Viewport|AddtoViewport _returnvalue 0)
  (bind _returnvalue_2 (UserInterface|CreateWidget "/Game/ProjectAmulet/UI/HUD/Widget_Compass.Widget_Compass_C" self))
  (UserInterface|Viewport|AddtoViewport _returnvalue_2 0)
  (bind _returnvalue_3 (UserInterface|CreateWidget "/Game/ProjectAmulet/UI/HUD/Widget_Objective.Widget_Objective_C" self (Variables|Default|GetWidget%20Text)))
  (UserInterface|Viewport|AddtoViewport _returnvalue_3 0))

(event Custom|ResetPlayerLocation
  (params (Location :type Vector))
  (bind _asthird_person_character (Utilities|Casting|CastToThirdPersonCharacter (Pawn|GetControlledPawn)))
  (Default|ResetPlayer _asthird_person_character Location))

(event EventTick
  (params (DeltaSeconds :type Float%20%28single-precision%29))
  ;[1 1 1] Compass Bearing
  (bind _asthird_person_character (Utilities|Casting|CastToThirdPersonCharacter (Pawn|GetControlledPawn)))
  (Default|CallCallUpdateCompass (* (.yaw (Math|Conversions|RotationFromXVector (Math|Transform|InverseTransformLocation (Transformation|GetWorldTransform (Variables|/Script/Engine.Character|GetMesh _asthird_person_character)) (Variables|Default|GetAmuletLocation)))) -1.0)))

(fn ConstructionScript)

(fn GameplayPCref
  (return self))