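; Gameplay player controller that loads player info, shows the starting objective and relays chat in networked play.
; On BeginPlay the local controller clears widgets, passes settings from the Steam game instance to PassCharacterInfoToServer, shows the "Explore the island." objective and sets game-only input.
; Chat text goes to the gameplay game mode with an empty sender name.
; SetupUI is a stub, and chat widget creation is disconnected, leaving UpdateChatWindow's target unset.
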(event Custom|GetChatMessage
  (params (TextToSend :type Text))
  ;[1 1 1] Gets chat message and sender name (no sender name since we dont have save / load game and the player info that comes with it)
  (Variables|Default|SetSenderText TextToSend)
  (Variables|Default|SetSenderName "")
  (bind _gameplaygmref (Class|BPIGamePlayGM|GameplayGMRef(Message) (Game|GetGameMode)))
  (Default|UpdateChat _gameplaygmref (Variables|Default|GetSenderName) (Variables|Default|GetSenderText)))

(event Custom|PassCharacterInfoToServer
  (params (Player%20Settings :type S%20Player%20Info%20Structure))
  ;[1 1 1] Passing loaded info to server
  (Variables|Default|SetPlayerSettingsSave Player%20Settings)
  (Utilities|FlowControl|Delay 0.5)
  (CallFunction|SetupUI))

(event Custom|SetupUI
  ;[1 1 1] Change this to setup the in game UI later
)

(event Custom|UpdateChatWindow
  (params (Sender :type Text) (Text :type Text))
  (Default|UpdateChatWindow (Variables|Default|GetGameplayChatWidget) Sender Text))

(event EventBeginPlay
  (if (Pawn|IsLocalController)
    (Viewport|RemoveAllWidgets)
    (bind _gameinstance (Class|BPIGameInstance|SteamGameInstanceRef(Message) (Game|GetGameInstance)))
    (bind _playerinfo (Default|GetPlayerInfo _gameinstance))
    (bind _output_get (Variables|Default|SetPlayerSettingsSave _playerinfo))
    (Utilities|FlowControl|Delay 0.2)
    (CallFunction|PassCharacterInfotoServer _output_get)
    (bind _returnvalue (UserInterface|CreateWidget "/Game/ProjectAmulet/UI/HUD/Widget_Objective.Widget_Objective_C"))
    (Variables|/Game/ProjectAmulet/UI/HUD/Widget_Objective.Widget_Objective_C|SetObjectiveMessage _returnvalue "Explore the island.")
    (UserInterface|Viewport|AddtoViewport _returnvalue 0)
    (Input|SetInputModeGameOnly (Game|GetPlayerController 0))))

(event Input|ActionEvents|InputActionChat
  (params (Key :type Key%20Structure))
  ;[1 1 1] Bring up mouse to use chat menu
  (:Pressed
    (Utilities|FlowControl|FlipFlop
      (:A
        (Variables|Default|SetbShowMouseCursor true))
      (:B
        (Variables|Default|SetbShowMouseCursor false)))))

(fn ConstructionScript)

(fn GameplayPCref
  (return self))