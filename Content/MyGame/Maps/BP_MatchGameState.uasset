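; BP_MatchGameState is a match game state that tracks which team, Alpha or Bravo, is attacking and how many wins each has.
; EarnAttackerPoint and EarnDefenderPoint use the current AttackingTeam to increment either AlphaWins or BravoWins.
; SwapTeams alternates the attacking side, starting with Alpha when none is set.
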(event EventBeginPlay)

(event EventTick
  (params (DeltaSeconds :type Float%20%28single-precision%29)))

(fn ConstructionScript)

(fn EarnAttackerPoint
  (switch Utilities|FlowControl|Switch|SwitchonBP_ETeam (Variables|Default|GetAttackingTeam)
    (:NewEnumerator0
      (bind _result (Math|Integer|IncrementInt (Variables|Default|GetAlphaWins))
        (:%20%20
          (Variables|Default|SetAlphaWins _result))))
    (:NewEnumerator1
      (bind _result_2 (Math|Integer|IncrementInt (Variables|Default|GetBravoWins))
        (:%20%20
          (Variables|Default|SetBravoWins _result_2))))))

(fn EarnDefenderPoint
  (switch Utilities|FlowControl|Switch|SwitchonBP_ETeam (Variables|Default|GetAttackingTeam)
    (:NewEnumerator0
      (bind _result (Math|Integer|IncrementInt (Variables|Default|GetBravoWins))
        (:%20%20
          (Variables|Default|SetBravoWins _result))))
    (:NewEnumerator1
      (bind _result_2 (Math|Integer|IncrementInt (Variables|Default|GetAlphaWins))
        (:%20%20
          (Variables|Default|SetAlphaWins _result_2))))))

(fn SwapTeams
  (switch Utilities|FlowControl|Switch|SwitchonBP_ETeam (Variables|Default|GetAttackingTeam)
    (:NewEnumerator2
      (Variables|Default|SetAttackingTeam "NewEnumerator0" :!label _label))
    (:NewEnumerator0
      (Variables|Default|SetAttackingTeam "NewEnumerator1"))
    (:NewEnumerator1
      (goto _label))))