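; Main menu player controller that gathers the local player's Steam identity and online friends for the game instance.
; Shortly after BeginPlay, it logs whether Steam is present, reads the player name either way, fetches the avatar and saves both as player info.
; It then asynchronously retrieves the friends list, fetches avatars for online friends and forwards each to the game instance through message calls.
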(event EventBeginPlay
  (bind _returnvalue (Game|GetGameInstance))
  (Utilities|FlowControl|Delay 0.2)
  (if (Class|AdvancedSessionsLibrary|HasOnlineSubsystem "STEAM")
    (Development|PrintString "Steam Is There")
    (Variables|Default|SetSteamName (Utilities|Text|ToText(String) (Class|AdvancedSessionsLibrary|GetPlayerName self)))
    (else
      (Development|PrintString "Steam Is Not There")
      (Variables|Default|SetSteamName (Utilities|Text|ToText(String) (Class|AdvancedSessionsLibrary|GetPlayerName self)))))
  (bind _returnvalue_2 (Class|AdvancedSteamFriendsLibrary|GetSteamFriendAvatar (Class|AdvancedSessionsLibrary|GetUniqueNetID self) "SteamAvatar_Medium")
    (:OnSuccess
      (Utilities|Struct|SetmembersinS_PlayerInfo (Variables|Default|GetPlayerInfo) (Variables|Default|GetSteamName) _returnvalue_2)
      (Class|BPIGameInstance|SavePlayerInfo(Message) _returnvalue (Variables|Default|GetPlayerInfo))
      (Class|BPIGameInstance|MainMenuPlayerInfo(Message) _returnvalue)
      (bind _results (|GetandStoreFriendsList (Game|GetPlayerController 0))
        (:OnSuccess
          (for _array_element _results
            (if (.bIsOnline (Utilities|Struct|BreakBPFriendPresenceInfo (.PresenceInfo (Utilities|Struct|BreakBPFriendInfo _array_element))))
              (bind _returnvalue_3 (Class|AdvancedSteamFriendsLibrary|GetSteamFriendAvatar (.UniqueNetId (Utilities|Struct|BreakBPFriendInfo _array_element)) "SteamAvatar_Medium")
                (:OnSuccess
                  (Class|BPIGameInstance|UpdateFriendList(Message) (Game|GetGameInstance) _array_element _returnvalue_3))))))))))

(fn ConstructionScript)