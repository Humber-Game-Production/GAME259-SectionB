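; Multiplayer lobby GameMode that tracks connected players, syncs host-selected map settings and server-travels to the match.
; PostLogin registers controllers and passes them Steam game instance server info, using interface messages throughout.
; EveryoneUpdate rebroadcasts player info, refreshes the host's kick list and checks character selection for start readiness.
; It also handles kicks, logouts, loading screens and character respawns at random PlayerStarts; travel map paths are unfinished placeholders.
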(event Custom|SpawnPlayer
  (params (Player :type Player%20Controller%20Object%20Reference)))

(event Custom|StartLoadingScreen
  ;[1 1 1] Will show loading screen and launch selected level
  (for _array_element (Variables|Default|GetConnectedPlayers)
    (bind _lobbypc (Class|BPILobbyPlayerController|LobbyPCRef(Message) _array_element))
    (Class|BPIGameInstance|ShowLoadingScreen(Message) _lobbypc))
  (CallFunction|LaunchGame))

(event Custom|HostUpdateGameSettings
  (params (SelectedMapImage :type Texture%202D%20Object%20Reference) (SelectedMapName :type Text) (SelectedMapTime :type Text) (SelectedMapID :type Integer))
  ;[1 1 1] Updates clients to update when server makes changes
  (Variables|Default|SetSelectedMapImage SelectedMapImage)
  (Variables|Default|SetSelectedMapName SelectedMapName)
  (Variables|Default|SetSelectedMapTime SelectedMapTime)
  (Variables|Default|SetSelectedMapID SelectedMapID)
  (for _array_element (Variables|Default|GetConnectedPlayers)
    (bind _lobbypc (Class|BPILobbyPlayerController|LobbyPCRef(Message) _array_element))
    (Default|UpdateLobbySettings _lobbypc (Variables|Default|GetSelectedMapImage) (Variables|Default|GetSelectedMapName) (Variables|Default|GetSelectedMapTime))))

(event Custom|PlayerKicked
  (params (PlayerID :type Integer))
  ;[1 1 1] Kicks selected player
  (bind _lobbypc (Class|BPILobbyPlayerController|LobbyPCRef(Message) (Utilities|Array|Get(acopy) (Variables|Default|GetConnectedPlayers) PlayerID)))
  (Default|Kicked _lobbypc))

(event Custom|EveryoneUpdate
  (bind _connectedplayers (Variables|Default|GetConnectedPlayers))
  ;[1 1 1] Updates most information every time someone connects
  (bind _output_get (Variables|Default|SetCurrentPlayers (Utilities|Array|Length (Variables|Default|GetConnectedPlayers))))
  (if (> _output_get 0)
    (Utilities|Array|Clear (Variables|Default|GetConnectedPlayersInfo))
    (for _array_element _connectedplayers
      (bind _lobbypc (Class|BPILobbyPlayerController|LobbyPCRef(Message) _array_element))
      (Utilities|Array|AddUnique (Variables|Default|GetConnectedPlayersInfo) (Variables|/Game/MyGame/Core/Networking/Lobby/BP_LobbyPC.BP_LobbyPC_C|GetPlayerSettings _lobbypc))
      (Default|UpdateNumberOfPlayers _lobbypc (Variables|Default|GetCurrentPlayers) (Variables|Default|GetMax%20Players)))
    (for _array_element_2 _connectedplayers
      (bind _lobbypc_2 (Class|BPILobbyPlayerController|LobbyPCRef(Message) _array_element_2))
      (Default|AddPlayerInfo _lobbypc_2 (Variables|Default|GetConnectedPlayersInfo))
      (CallFunction|AddtoKickList))
    (bind _array_element_3 (Utilities|Array|ForEachLoopwithBreak (Variables|Default|GetConnectedPlayersInfo))
      (:LoopBody
        (if (== (Utilities|Struct|BreakS_PlayerInfo _array_element_3) 0)
          (Variables|Default|SetCanWeStart false)
          (CallFunction|CannotStartGame)
          (else
            (Variables|Default|SetCanWeStart true)))))))

(event Custom|AddToKickList
  ;[1 1 1] Adds players to kick list
  (bind _lobbypc (Class|BPILobbyPlayerController|LobbyPCRef(Message) (Game|GetPlayerController 0)))
  (Default|AddPlayertoKickWindow _lobbypc))

(event Custom|CannotStartGame
  (Utilities|Array|ForEachLoopwithBreak (Variables|Default|GetConnectedPlayersInfo)) ; enters at Break
)

(event Custom|ChangeCharacter
  (params (ConnectedPlayer :type Player%20Controller%20Object%20Reference) (CharacterClass :type Character%20Class%20Reference) (ChangedStatus :type Boolean))
  (bind _returnvalue (Pawn|GetControlledPawn ConnectedPlayer))
  (bind _spawnpoints (Variables|Default|GetSpawnPoints))
  ;[1 1 1] Spawn the selected character that the player chose. (will spawn with the class given)
  (if (not ChangedStatus)
    (Utilities|IsValid _returnvalue
      (:Is%20Valid
        (Actor|DestroyActor _returnvalue))
      (:Is%20Not%20Valid
        _))
    (bind _returnvalue_2 (Game|SpawnActorfromClass CharacterClass (Transformation|GetActorTransform (Utilities|Array|Get(acopy) _spawnpoints (Math|Random|RandomIntegerinRange 0 (- (Utilities|Array|Length _spawnpoints) 1)))) "AlwaysSpawn" 0 0))
    (Pawn|Possess ConnectedPlayer _returnvalue_2)))

(event Custom|LaunchGame
  (bind _returnvalue (Game|GetPlayerController 0))
  (switch int (Variables|Default|GetSelectedMapID)
    (:0
      ;[1 1 1] This needs to be changed to location of maps when we have them
      (Development|ExecuteConsoleCommand "servertravel /Game/MyGame/Maps/" _returnvalue))
    (:1
      (Development|ExecuteConsoleCommand "servertravel /Game/MyGame/Maps/" _returnvalue))))

(event EventOnLogout
  (params (ExitingController :type Controller%20Object%20Reference))
  (bind _connectedplayers (Variables|Default|GetConnectedPlayers))
  ;[1 1 1] Removes player info when disconnected (if there will be character selection, important work will need to be added here to free up characters)
  (bind (_array_element _array_index) (Utilities|Array|ForEachLoopwithBreak _connectedplayers :!label _label)
    (:LoopBody
      (if (== ExitingController _array_element)
        (goto _label Break)))
    (:Completed
      (Class|BPILobbyPlayerController|LobbyPCRef(Message) (Utilities|Array|Get(acopy) _connectedplayers _array_index))
      (Utilities|Array|RemoveIndex (Variables|Default|GetConnectedPlayers) _array_index)
      (Utilities|Array|RemoveIndex (Variables|Default|GetConnectedPlayersInfo) _array_index)
      (CallFunction|EveryoneUpdate))))

(event EventPostLogin
  (params (NewPlayer :type Player%20Controller%20Object%20Reference))
  ;[1 1 1] Initial setup that runs when someone connects
  (bind _output_get (Variables|Default|SetConnectedPlayer NewPlayer))
  (Utilities|Array|AddUnique (Variables|Default|GetConnectedPlayers) _output_get)
  (bind _outactors (Actor|GetAllActorsOfClass "/Script/Engine.PlayerStart"))
  (Variables|Default|SetSpawnPoints _outactors)
  (bind _gameinstance (Class|BPIGameInstance|SteamGameInstanceRef(Message) (Game|GetGameInstance)))
  (Variables|Default|SetServer%20Name (Variables|/Game/MyGame/Core/Networking/SteamGameInstance.SteamGameInstance_C|GetServerName _gameinstance))
  (Variables|Default|SetMax%20Players (Variables|/Game/MyGame/Core/Networking/SteamGameInstance.SteamGameInstance_C|GetMaxPlayers _gameinstance))
  (bind _lobbypc (Class|BPILobbyPlayerController|LobbyPCRef(Message) (Variables|Default|GetConnectedPlayer)))
  (bind _output_get_2 (Variables|Default|SetLobby%20PC _lobbypc))
  (Default|InitialSetup _output_get_2 (Variables|Default|GetServer%20Name) (Variables|Default|GetSelectedMapImage) (Variables|Default|GetSelectedMapName) (Variables|Default|GetSelectedMapTime)))

(fn ConstructionScript)

(fn LobbyGMRef
  (return self))