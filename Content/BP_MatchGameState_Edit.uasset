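; Game state for a two-team attack/defend amulet match, tracking rounds, scores, team lives and amulet points.
; Changes are broadcast through event dispatchers, and one timer handle drives pre-round and round countdowns, with expiry of the round scoring for defenders.
; IncrementRound swaps teams at halftime, resets amulet spawns, shows round or overtime screens and signals match end.
; It delegates pre-round start, round end and player relocation to BP_MatchGameMode.
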(event Custom|CheckTimer
  (Networking|SwitchHasAuthority
    (:Authority
      (CallFunction|Timers))
    (:Remote
      (CallFunction|Timer(Server)))))

(event Custom|Timer%20%28Server%29
  (CallFunction|Timers))

(event Custom|ScoreUpdate
  ;[1 1 1] Event Dispatcher events
  (Default|CallUpdateScore))

(event Custom|Timers
  ;[1 1 1] Event Dispatcher events
  (Default|CallUpdateTimers))

(event Custom|AlphaLifeCount
  ;[1 1 1] Event Dispatcher events
  (Default|CallUpdateAlphaLives))

(event Custom|BravoLifeCount
  ;[1 1 1] Event Dispatcher events
  (Default|CallUpdateBravoLives))

(event Custom|MatchEnd
  ;[1 1 1] Event Dispatcher events
  (Default|CallEndOfMatch))

(event Custom|ResetRound
  ;[1 1 1] Event Dispatcher events
  (Default|CallRoundReset))

(event Custom|AmuletPoints
  ;[1 1 1] Event Dispatcher events
  (Default|CallUpdateAmuletPoints))

(event EventBeginPlay)

(event EventTick
  (params (DeltaSeconds :type Float%20%28single-precision%29))
  (CallFunction|Timers))

(fn ConstructionScript)

(fn EarnAttackerPoint
  (CallFunction|AddScore true))

(fn EarnDefenderPoint
  (CallFunction|AddScore false)
  (bind _asbp_match_game_mode (Utilities|Casting|CastToBP_MatchGameMode (Game|GetGameMode)))
  (Default|EndRound _asbp_match_game_mode))

(fn SwapTeams
  (Development|PrintString "Teams Swaped")
  (switch Utilities|FlowControl|Switch|SwitchonBP_ETeam (Variables|Round|GetAttackingTeam)
    (:NewEnumerator0
      (Variables|Round|SetAttackingTeam "NewEnumerator1"))
    (:NewEnumerator1
      (Variables|Round|SetAttackingTeam "NewEnumerator0")))
  (Networking|SwitchHasAuthority
    (:Authority
      (bind _asbp_match_game_mode (Utilities|Casting|CastToBP_MatchGameMode (Game|GetGameMode)))
      (Default|SwapTeams _asbp_match_game_mode)
      (CallFunction|SwapAmuletViewers)
      (Default|ResetPlayerLocations _asbp_match_game_mode)
      ;[1 1 1] Set objective messages depending on team
      (bind _asbp_gameplay_pc (Utilities|Casting|CastToBP_GameplayPC (Game|GetPlayerController 0)))
      (Variables|/Game/ProjectAmulet/Core/Networking/Gameplay/BP_GameplayPC.BP_GameplayPC_C|SetWidget%20Text _asbp_gameplay_pc "Retrieve the amulet!")
      (Variables|Round|SetCurrentAmuletPoints (Variables|Round|GetStartingAmuletPoints))
      (CallFunction|AmuletPoints))))

(fn GetRemainingTimeMinSec
  (bind _timer (Variables|Round|GetTimer))
  (bind _returnvalue (Utilities|Time|GetTimerRemainingTimebyHandle _timer))
  (bind (_remainder _returnvalue_2) (Math|Float|Division(WholeandRemainder) _returnvalue 6e+01))
  (return _returnvalue_2 (Math|Float|Truncate _remainder)))

(fn AlphaLoseLife
  (bind _alphalives (Variables|Score|GetAlphaLives))
  (Math|Integer|DecrementInt _alphalives
    (:%20%20
      (CallFunction|AlphaLifeCount)
      (return (== _alphalives 0)))))

(fn BravoLoseLife
  (bind _bravolives (Variables|Score|GetBravoLives))
  (Math|Integer|DecrementInt _bravolives
    (:%20%20
      (CallFunction|BravoLifeCount)
      (return (== _bravolives 0)))))

(fn IncrementRound
  (params (Halftime :type Integer) (FinalRound :type Integer))
  (bind _currentround (Variables|Round|GetCurrentRound))
  (if (< _currentround FinalRound)
    (if (== _currentround Halftime)
      (CallFunction|SwapTeams))
    (Math|Integer|IncrementInt (Variables|Round|GetCurrentRound)
      (:%20%20
        (CallFunction|ResetAmuletSystem)
        (bind _asbp_match_game_mode (Utilities|Casting|CastToBP_MatchGameMode (Game|GetGameMode)))
        (Default|StartPreRound _asbp_match_game_mode)
        ;[1 1 1] Add Round Screen Widgets Depending on Current Round
        ;;[1 1 1] Round 1
        (Development|PrintString "Started Round")
        (if (== (Variables|Round|GetCurrentRound) 1)
          (bind _returnvalue (UserInterface|CreateWidget "/Game/ProjectAmulet/UI/HUD/WIdget_RoundScreen.WIdget_RoundScreen_C" (Game|GetPlayerController 0)))
          (Class|UserWidget|PlayAnimationForward _returnvalue (Variables|/Game/ProjectAmulet/UI/HUD/WIdget_RoundScreen.WIdget_RoundScreen_C|GetRound1_Fade _returnvalue) 1.0 false)
          (UserInterface|Viewport|AddtoViewport _returnvalue 0)
          (else
            ;;[1 1 1] Round 2
            (if (== (Variables|Round|GetCurrentRound) 2)
              (bind _returnvalue_2 (UserInterface|CreateWidget "/Game/ProjectAmulet/UI/HUD/WIdget_RoundScreen.WIdget_RoundScreen_C" (Game|GetPlayerController 0)))
              (Class|UserWidget|PlayAnimationForward _returnvalue_2 (Variables|/Game/ProjectAmulet/UI/HUD/WIdget_RoundScreen.WIdget_RoundScreen_C|GetRound2_Fade _returnvalue_2) 1.0 false)
              (UserInterface|Viewport|AddtoViewport _returnvalue_2 0)
              (else
                ;;[1 1 1] Overtime
                (if (== (Variables|Round|GetCurrentRound) 3)
                  (bind _returnvalue_3 (UserInterface|CreateWidget "/Game/ProjectAmulet/UI/HUD/WIdget_RoundScreen.WIdget_RoundScreen_C" (Game|GetPlayerController 0)))
                  (Class|UserWidget|PlayAnimationForward _returnvalue_3 (Variables|/Game/ProjectAmulet/UI/HUD/WIdget_RoundScreen.WIdget_RoundScreen_C|GetOvertime_Fade _returnvalue_3) 1.0 false)
                  (UserInterface|Viewport|AddtoViewport _returnvalue_3 0)
                  ;[1 1 1] Set overtime objective message
                  (bind _asbp_gameplay_pc (Utilities|Casting|CastToBP_GameplayPC (Game|GetPlayerController 0)))
                  (Variables|/Game/ProjectAmulet/Core/Networking/Gameplay/BP_GameplayPC.BP_GameplayPC_C|SetWidget%20Text _asbp_gameplay_pc "Kill the enemy team!"))))))))
    (else
      (Development|PrintString "END OF MATCH")
      (CallFunction|MatchEnd))))

(fn UseAmuletPoints
  (params (PointsToUse :type Integer))
  (if (<= PointsToUse (Variables|Round|GetCurrentAmuletPoints))
    (Variables|Round|SetCurrentAmuletPoints (- (Variables|Round|GetCurrentAmuletPoints) PointsToUse))
    (CallFunction|AmuletPoints))
  (return (<= PointsToUse (Variables|Round|GetCurrentAmuletPoints))))

(fn AddScore
  (params (IsAlpha :type Boolean))
  (if IsAlpha
    (Math|Integer|IncrementInt (Variables|Score|GetAlphaWins)
      (:%20%20
        _))
    (else
      (Math|Integer|IncrementInt (Variables|Score|GetBravoWins)
        (:%20%20
          _))))
  (CallFunction|ScoreUpdate))

(fn StartPreRoundTimer
  (params (Duration :type Float%20%28single-precision%29) (FunctionName :type String))
  (bind _asbp_match_game_mode (Utilities|Casting|CastToBP_MatchGameMode (Game|GetGameMode)))
  (bind _returnvalue (Utilities|Time|SetTimerbyFunctionName _asbp_match_game_mode FunctionName Duration))
  (Variables|Round|SetTimer _returnvalue))

(fn StartRoundTimer
  (params (Duration :type Float%20%28single-precision%29))
  (bind _returnvalue (Utilities|Time|SetTimerbyFunctionName self "EarnDefenderPoint" Duration))
  (Variables|Round|SetTimer _returnvalue))

(fn ResetAmuletSystem
  (bind _outactors (Actor|GetAllActorsOfClass "/Game/ProjectAmulet/GameMode/EnvironmentBPs/AmuletSpawnLocation.AmuletSpawnLocation_C"))
  (bind _output_get (Variables|Round|SetAmuletLocations _outactors))
  (for _array_element _output_get
    (Default|ResetAmuletLocation _array_element)))

(fn SwapAmuletViewers
  (for _array_element (Variables|Round|GetAmuletLocations)
    (Default|SwitchVisability _array_element)))