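; Match game mode for a round-based attack/defend mode with amulet spawn locations, team swapping and respawns.
; Pre-round respawns everyone, freezes attackers and activates amulet locations; the main round unfreezes attackers, locks locations and deducts occupied ones' defense cost.
; Rounds end on WinCon results or lost team lives, with scoring, timers and round increments delegated to BP_MatchGameState.
; Players spawn at Attacker/Defender-tagged PlayerStarts matched to their team.
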(event Custom|FreezeAttackers
  (params (bNewMoveInput :type Boolean))
  (for _array_element (Variables|Default|GetAttackingTeam)
    (bind _asbp_gameplay_pc (Utilities|Casting|CastToBP_GameplayPC _array_element))
    (Default|SetFrozen _asbp_gameplay_pc bNewMoveInput)))

(event Custom|ResetRound
  (CallFunction|WinReset))

(event EventBeginPlay
  (Default|IncrementRound (Variables|Default|GetGameStateRef) (Variables|Default|GetHalftimeRound) (Variables|Default|GetFinalRound)))

(fn ConstructionScript)

(fn EarnPointAttackers
  (bind _asbp_match_game_state (Utilities|Casting|CastToBP_MatchGameState (Game|GetGameState)))
  (Default|EarnAttackerPoint _asbp_match_game_state)
  (CallFunction|EndRound))

(fn EarnPointDefenders
  (bind _asbp_match_game_state (Utilities|Casting|CastToBP_MatchGameState (Game|GetGameState)))
  (Default|EarnDefenderPoint _asbp_match_game_state)
  (CallFunction|EndRound))

(fn EndRound
  (Variables|Default|SetbIsAttackPhase false)
  (Default|IncrementRound (Variables|Default|GetGameStateRef) (Variables|Default|GetHalftimeRound) (Variables|Default|GetFinalRound)))

(fn AlphaLoseLife
  (bind _asbp_match_game_state (Utilities|Casting|CastToBP_MatchGameState (Game|GetGameState)))
  (bind _iseliminated (Default|AlphaLoseLife _asbp_match_game_state))
  (if _iseliminated
    (CallFunction|EndRound)))

(fn BravoLoseLife
  (bind _asbp_match_game_state (Utilities|Casting|CastToBP_MatchGameState (Game|GetGameState)))
  (bind _iseliminated (Default|BravoLoseLife _asbp_match_game_state))
  (if _iseliminated
    (CallFunction|EndRound)))

(fn CheckAmuletLocation
  ;[1 1 1] Get Active Spawn Location and check point cost
  (bind _outactors (Actor|GetAllActorsOfClass "/Game/ProjectAmulet/GameMode/EnvironmentBPs/AmuletSpawnLocation.AmuletSpawnLocation_C"))
  (bind _output_get (LocalVariables|SetSpawnLocations _outactors))
  (for _array_element _output_get
    (Variables|/Game/ProjectAmulet/GameMode/EnvironmentBPs/AmuletSpawnLocation.AmuletSpawnLocation_C|SetSpawnLocationsActive? _array_element false)
    (if (Variables|/Game/ProjectAmulet/GameMode/EnvironmentBPs/AmuletSpawnLocation.AmuletSpawnLocation_C|GetAmuletSpawned? _array_element)
      (Variables|Default|SetDefensePoints (- (Variables|Default|GetDefensePoints) (Variables|/Game/ProjectAmulet/GameMode/EnvironmentBPs/AmuletSpawnLocation.AmuletSpawnLocation_C|GetDefenseCost _array_element))))))

(fn ActivateSpawnLocations
  (bind _outactors (Actor|GetAllActorsOfClass "/Game/ProjectAmulet/GameMode/EnvironmentBPs/AmuletSpawnLocation.AmuletSpawnLocation_C"))
  (bind _output_get (LocalVariables|SetSpawnLocations _outactors))
  (for _array_element _output_get
    (Variables|/Game/ProjectAmulet/GameMode/EnvironmentBPs/AmuletSpawnLocation.AmuletSpawnLocation_C|SetSpawnLocationsActive? _array_element true)))

(fn WinReset
  (bind _returnvalue (Actor|GetActorOfClass "/Game/ProjectAmulet/GameMode/EnvironmentBPs/WinCon.WinCon_C"))
  (if (Variables|/Game/ProjectAmulet/GameMode/EnvironmentBPs/WinCon.WinCon_C|GetWin? _returnvalue)
    (Scoring|EarnPointAttackers)
    (else
      (Scoring|EarnPointDefenders)))
  (CallFunction|EndRound)
  (Development|PrintString "reset level"))

(fn SetMatchTime
  (params (Time :type Float%20%28single-precision%29))
  (Variables|Default|SetMatchTime Time))

(fn StartPreRound
  ;[1 1 1] Starts the preperation phase of the round
  (CallFunction|ResetPlayerLocations)
  (CallFunction|FreezeAttackers true)
  (CallFunction|ActivateSpawnLocations)
  (Default|StartPreRoundTimer (Variables|Default|GetGameStateRef) (Variables|Default|GetPrePhaseTime) "StartRound"))

(fn StartRound
  ;[1 1 1] Starts the main round
  (CallFunction|FreezeAttackers false)
  (CallFunction|CheckAmuletLocation)
  (Default|StartRoundTimer (Variables|Default|GetGameStateRef) (Variables|Default|GetMatchTime)))

(fn ChoosePlayerStart
  (params (Player :type Controller%20Object%20Reference))
  (if (Variables|Default|GetFirstPlayerSpawned)
    _
    (else
      (Development|PrintString "Init")
      (CallFunction|InitSpawnPoints)))
  (bind _returnvalue (CallFunction|InitTeams Player))
  (Variables|Default|SetPlayersSpawned (+ (Variables|Default|GetPlayersSpawned) 1))
  (LocalVariables|SetNewSpawnLocation _returnvalue)
  (return (LocalVariables|GetNewSpawnLocation)))

(fn InitSpawnPoints
  (CallFunction|InitGameState)
  (bind _outactors (Actor|GetAllActorsOfClass "/Script/Engine.PlayerStart"))
  (bind _output_get (Variables|Default|SetSpawnPoints _outactors))
  (Variables|Default|SetPlayerStarts _output_get)
  (Variables|Default|SetFirstPlayerSpawned true)
  (for _array_element (Variables|Default|GetPlayerStarts)
    (switch name (Variables|/Script/Engine.PlayerStart|GetPlayerStartTag _array_element)
      (:Attacker
        (Utilities|Array|AddUnique (Variables|Default|GetAttackerSpawns) _array_element))
      (:Defender
        (Utilities|Array|AddUnique (Variables|Default|GetDefenderSpawns) _array_element)))))

(fn InitGameState
  (bind _asbp_match_game_state (Utilities|Casting|CastToBP_MatchGameState (Game|GetGameState)))
  (Variables|Default|SetGameStateRef _asbp_match_game_state))

(fn InitTeams
  (params (Player :type Controller%20Object%20Reference))
  (bind _playerstate (Variables|/Script/Engine.Controller|GetPlayerState Player))
  (for _array_element (Variables|Default|GetPlayerStarts)
    (switch name (Variables|/Script/Engine.PlayerStart|GetPlayerStartTag _array_element)
      (:Attacker
        (bind _asbp_match_player_state (Utilities|Casting|CastToBP_MatchPlayerState _playerstate))
        (if (Utilities|Enum|Equal(Enum) (Variables|/Game/ProjectAmulet/Maps/BP_MatchPlayerState.BP_MatchPlayerState_C|GetTeam _asbp_match_player_state) "NewEnumerator0")
          (bind _asbp_gameplay_pc (Utilities|Casting|CastToBP_GameplayPC Player))
          (Utilities|Array|AddUnique (Variables|Default|GetAttackingTeam) _asbp_gameplay_pc)
          (LocalVariables|SetNewSpawnLocation _array_element :!label _label)))
      (:Defender
        (bind _asbp_match_player_state_2 (Utilities|Casting|CastToBP_MatchPlayerState _playerstate))
        (if (Utilities|Enum|Equal(Enum) (Variables|/Game/ProjectAmulet/Maps/BP_MatchPlayerState.BP_MatchPlayerState_C|GetTeam _asbp_match_player_state_2) "NewEnumerator1")
          (bind _asbp_gameplay_pc_2 (Utilities|Casting|CastToBP_GameplayPC Player))
          (Utilities|Array|AddUnique (Variables|Default|GetDefendingTeam) _asbp_gameplay_pc_2)
          (goto _label)))))
  (Utilities|Array|RemoveItem (Variables|Default|GetPlayerStarts) (LocalVariables|GetNewSpawnLocation))
  (Utilities|IsValid (LocalVariables|GetNewSpawnLocation)
    (:Is%20Valid
      (return (LocalVariables|GetNewSpawnLocation)))
    (:Is%20Not%20Valid
      (Development|PrintString "Is Valid"))))

(fn RespawnPlayer
  (params (Controller :type Controller%20Object%20Reference))
  (bind _asbp_match_player_state (Utilities|Casting|CastToBP_MatchPlayerState (Variables|/Script/Engine.Controller|GetPlayerState Controller)))
  (if (Utilities|Enum|Equal(Enum) (Variables|/Game/ProjectAmulet/Maps/BP_MatchGameState.BP_MatchGameState_C|GetAttackingTeam (Variables|Default|GetGameStateRef)) (Variables|/Game/ProjectAmulet/Maps/BP_MatchPlayerState.BP_MatchPlayerState_C|GetTeam _asbp_match_player_state))
    (LocalVariables|SetSpawnPos (.OutItem (Utilities|Array|Random (Variables|Default|GetAttackerSpawns))))
    (else
      (LocalVariables|SetSpawnPos (.OutItem (Utilities|Array|Random (Variables|Default|GetDefenderSpawns))))))
  (return (LocalVariables|GetSpawnPos)))

(fn OnKill
  (params (Player :type Character%20Object%20Reference))
  (bind _output_get (LocalVariables|SetController (Pawn|GetController Player)))
  (Pawn|UnPossess _output_get)
  (bind _playerstart (CallFunction|RespawnPlayer (LocalVariables|GetController)))
  (Class|GameModeBase|RestartPlayeratPlayerStart (LocalVariables|GetController) _playerstart))

(fn InitPlayerHUD
  (params (Player :type Controller%20Object%20Reference))
  (bind _output_get (LocalVariables|SetConnectedPlayer Player))
  (bind _asbp_gameplay_pc (Utilities|Casting|CastToBP_GameplayPC _output_get))
  (Default|InitialSetup _asbp_gameplay_pc))

(fn ResetPlayerLocations
  (for _array_element (Variables|Default|GetAttackingTeam)
    (bind _asthird_person_character (Utilities|Casting|CastToThirdPersonCharacter (Pawn|GetControlledPawn _array_element)))
    (CallFunction|OnKill _asthird_person_character)
    (Actor|DestroyActor _asthird_person_character)
    (bind _asbp_match_player_state (Utilities|Casting|CastToBP_MatchPlayerState (Variables|/Script/Engine.Pawn|GetPlayerState _asthird_person_character)))
    (Default|RespawnUpdate _asbp_match_player_state))
  (for _array_element_2 (Variables|Default|GetDefendingTeam)
    (bind _asthird_person_character_2 (Utilities|Casting|CastToThirdPersonCharacter (Pawn|GetControlledPawn _array_element_2)))
    (CallFunction|OnKill _asthird_person_character_2)
    (Actor|DestroyActor _asthird_person_character_2)
    (bind _asbp_match_player_state_2 (Utilities|Casting|CastToBP_MatchPlayerState (Variables|/Script/Engine.Pawn|GetPlayerState _asthird_person_character_2)))
    (Default|RespawnUpdate _asbp_match_player_state_2)))

(fn SwapTeams
  ;[1 1 1] Reset's all the spawn points so when team's swap all the spawn points will too
  (LocalVariables|SetTempDefendingTeam (Variables|Default|GetDefendingTeam))
  (LocalVariables|SetTempAttackingTeam (Variables|Default|GetAttackingTeam))
  (Variables|Default|SetAttackingTeam (LocalVariables|GetTempDefendingTeam))
  (Variables|Default|SetDefendingTeam (LocalVariables|GetTempAttackingTeam)))